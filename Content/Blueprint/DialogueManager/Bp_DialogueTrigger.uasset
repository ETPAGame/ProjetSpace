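; A trigger volume actor that plays dialogue audio the first time the first-person character enters its box.
; The overlap passes the trigger's IdTrigger to PlayAudio on BP_DialogueManager, gated by a DoOnce.
; The construction script finds the manager in the level, caches it and adds to its TriggerRef list.
; It also snaps a spline point to the manager's location, visually linking the two actors.
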(event `self.Box.OnComponentBeginOverlap`
  (params (OverlappedComponent :type "PrimitiveComponent Object Reference") (OtherActor :type "Actor Object Reference") (OtherComp :type "PrimitiveComponent Object Reference") (OtherBodyIndex :type Integer) (bFromSweep :type Boolean) (SweepResult :type "HitResult Structure (by ref)"))
  (cast `/Game/Blueprint/BP_FirstPersonCharacter` OtherActor)
  (`/Engine/EditorBlueprintResources/StandardMacros.DoOnce` false
    (:`Completed`
      (`/Game/Blueprint/DialogueManager/BP_DialogueManager.PlayAudio` (`self.DialogueManager`) (`self.IdTrigger`)))))

(fn `UserConstructionScript`
  (bind _returnvalue (`GameplayStatics.GetActorOfClass` "/Game/Blueprint/DialogueManager/BP_DialogueManager.BP_DialogueManager_C"))
  (`KismetArrayLibrary.Array_AddUnique` (`/Game/Blueprint/DialogueManager/BP_DialogueManager.TriggerRef` _returnvalue))
  (set `self.DialogueManager` _returnvalue)
  (`SplineComponent.SetLocationAtSplinePoint` (`self.Spline`) 1 (`self.K2_GetActorLocation` (`self.DialogueManager`)) "World" true))