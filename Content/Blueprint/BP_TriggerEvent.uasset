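; One-shot trigger volume that, when enabled and overlapped by the player, zero-G pawn or monster, messages its WiredItems through BPI_WiredActor.
; Optional flags add a reactor alarm and voice sequence ahead of the trigger, a low-oxygen call on the character, and a HUD glyph switch.
; WiredAction enables it, and ResetActor re-arms both DoOnce gates.
; The construction script draws splines to wired actors to visualize links.
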(event `Reset`
  (goto _label :!via `Reset`))

(event `self.Box.OnComponentBeginOverlap`
  (params (OverlappedComponent :type "PrimitiveComponent Object Reference") (OtherActor :type "Actor Object Reference") (OtherComp :type "PrimitiveComponent Object Reference") (OtherBodyIndex :type Integer) (bFromSweep :type Boolean) (SweepResult :type "HitResult Structure (by ref)"))
  (if (`self.Enabled?`)
    (if (`self.SoundGeneratorOn?`)
      (`/Engine/EditorBlueprintResources/StandardMacros.DoOnce` false :!label _label
        (:`Completed`
          (`GameplayStatics.PlaySound2D` "/Game/Audio/SFX/Environment/Reactor/DownReactor_SciFi_01_alarmOn.DownReactor_SciFi_01_alarmOn" 0.5 1.0 0.0 null null)
          (`KismetSystemLibrary.Delay` 0.75)
          (`GameplayStatics.PlaySound2D` "/Game/Audio/Dialogue/Tess/Tess_GravityOff.Tess_GravityOff" 1.0 1.0 0.0 null null)
          (`|ExecutionSequence`
            (:`then_0`
              (`KismetSystemLibrary.Delay` 2.0)
              (`GameplayStatics.PlaySound2D` "/Game/Audio/Dialogue/Karl/Dial_Karl_React_WhyHaveToDoThis.Dial_Karl_React_WhyHaveToDoThis" 1.0 1.0 0.0 null null))
            (:`then_1`
              (bind _asbp_first_person_character (cast `/Game/Blueprint/BP_FirstPersonCharacter` OtherActor :!label _label_2)
                (:`then`
                  _)
                (:`CastFailed`
                  (cast `/Game/Blueprint/BP_ZeroGPawnCam` OtherActor
                    (:`then`
                      _)
                    (:`CastFailed`
                      (cast `/Game/Monster/BP_Monster` OtherActor)))))
              (`/Engine/EditorBlueprintResources/StandardMacros.DoOnce` false :!label _label_3
                (:`Completed`
                  (for _array_element (`self.WiredItems`)
                    (if (`KismetSystemLibrary.DoesImplementInterface` _array_element "/Game/Blueprint/BPI_WiredActor.BPI_WiredActor_C")
                      (message `/Game/Blueprint/BPI_WiredActor.WiredAction` _array_element)))
                  (if (`self.TriggerLow?`)
                    (`/Game/Blueprint/BP_FirstPersonCharacter.OxygenLow` _asbp_first_person_character))
                  (if (`self.TriggerGlyphe?`)
                    (bind _asbp_player_controller (cast `/Game/Blueprint/BP_PlayerController` (`GameplayStatics.GetPlayerController` 0)))
                    (`/Game/UserInterface/WPB_HUDInGame.SwitchBetweenGlypheAndNoGlyphe` (`/Game/Blueprint/BP_PlayerController.HUDRef` _asbp_player_controller) (`self.GlypheOn?`)))))))))
      (else
        (goto _label_2)))))

(event `Reset2`
  (goto _label_3 :!via `Reset`))

(event `/Game/Blueprint/BPI_WiredActor.WiredAction`
  (set `self.Enabled?` true))

(event `/Game/Blueprint/BPI_WiredActor.ResetActor`
  (set `self.Enabled?` true)
  (`self.Reset`)
  (`self.Reset2`))

(fn `UserConstructionScript`
  ;[1 0.5141 0.9922] Draw Link
  (for _array_element (`self.WiredItems`)
    (`/Engine/EditorBlueprintResources/StandardMacros.IsValid` _array_element
      (:`Is Valid`
        (bind _returnvalue (`AddComponent|NODE_AddSplineComponent-0`))
        (`SplineComponent.SetSplinePoints` _returnvalue (`|MakeArray` (`self.K2_GetActorLocation` _array_element) (`SceneComponent.K2_GetComponentLocation` (`self.Billboard`))) "World" true)))))