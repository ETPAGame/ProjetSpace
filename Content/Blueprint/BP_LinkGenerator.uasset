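; Generator actor that links to the actors in its WiredStaticMesh array and triggers color changes on wired cables.
; The construction script draws each link as a new two-point world-space spline from each valid actor to the generator's root.
; The WiredAction event loops over the same array, casts elements to BP_PlaneCable and calls Color with each array index.
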(event `/Game/Blueprint/BPI_WiredActor.WiredAction`
  (for (_array_element _array_index) (`self.WiredStaticMesh`)
    (bind _asbp_plane_cable (cast `/Game/Blueprint/BP_PlaneCable` _array_element))
    (`/Game/Blueprint/BP_PlaneCable.Color` _asbp_plane_cable (`KismetMathLibrary.Conv_IntToDouble` _array_index))))

(fn `UserConstructionScript`
  ;[1 0.5141 0.9922] Draw Link
  (for _array_element (`self.WiredStaticMesh`)
    (`/Engine/EditorBlueprintResources/StandardMacros.IsValid` _array_element
      (:`Is Valid`
        (bind _returnvalue (`AddComponent|NODE_AddSplineComponent-0`))
        (`SplineComponent.SetSplinePoints` _returnvalue (`|MakeArray` (`self.K2_GetActorLocation` _array_element) (`SceneComponent.K2_GetComponentLocation` (`self.DefaultSceneRoot`))) "World" true)))))