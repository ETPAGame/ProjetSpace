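; BP_LayeredDoor is an automatic multi-panel door that opens while the first-person character is inside its Box trigger and closes when they leave.
; One DoorMovement timeline, played or reversed, lerps the front and back panels vertically and slides the two middle panels apart sideways.
; Stored audio components let each direction stop the other's hangar sound, and a closing sound plays if CloseSound is still playing when the timeline finishes.
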(event `Open`
  (bind _returnvalue (`SceneComponent.K2_GetComponentLocation` (`self.Box`)))
  (bind _returnvalue_2 (`AudioComponent.IsPlaying` (`self.CloseSound`)))
  ;[1 1 1] SD
  (bind _returnvalue_3 (`GameplayStatics.SpawnSoundAtLocation` "/Game/Audio/SFX/Environment/Door/SC_Door_Hangar_1.SC_Door_Hangar_1" _returnvalue (struct) 0.5 1.0 0.0 "/Game/Audio/AttenuationVolume/AV_MonsterFootstep.AV_MonsterFootstep" null))
  (bind _output_get (set `self.OpenSound` _returnvalue_3))
  (if _returnvalue_2
    (`AudioComponent.Stop` (`self.CloseSound`))
    (bind (_direction _alpha) (`Timeline|DoorMovement` :!label _label)
      (:`Update`
        (bind _returnvalue_4 (`KismetMathLibrary.Lerp` 180.0 525.0 _alpha))
        (`SceneComponent.K2_SetRelativeLocation` (`self.FrontDoor`) (`KismetMathLibrary.MakeVector` 15.0 0.0 _returnvalue_4) false false)
        (`SceneComponent.K2_SetRelativeLocation` (`self.BackDoor`) (`KismetMathLibrary.MakeVector` -15.0 0.0 _returnvalue_4) false false)
        (bind _returnvalue_5 (`KismetMathLibrary.Lerp` 117.0 325.0 _alpha))
        (`SceneComponent.K2_SetRelativeLocation` (`self.MiddleDoorL`) (`KismetMathLibrary.MakeVector` 0.0 _returnvalue_5 180.0) false false)
        (`SceneComponent.K2_SetRelativeLocation` (`self.MiddleDoorR`) (`KismetMathLibrary.MakeVector` 0.0 (* _returnvalue_5 -1.0) 180.0) false false))
      (:`Finished`
        (if _returnvalue_2
          (`AudioComponent.Stop` (`self.CloseSound`))
          (`GameplayStatics.PlaySoundAtLocation` "/Game/Audio/SFX/Environment/Door/SC_Door_Hangar_Closing_1.SC_Door_Hangar_Closing_1" _returnvalue (struct) 0.2 1.0 0.0 "/Game/Audio/AttenuationVolume/AV_MonsterFootstep.AV_MonsterFootstep" null null null))))
    (else
      (goto _label))))

(event `Close`
  ;[1 1 1] SD
  (`AudioComponent.Stop` (stale `Open` _output_get))
  (bind _returnvalue (`GameplayStatics.SpawnSoundAtLocation` "/Game/Audio/SFX/Environment/Door/SC_Door_Hangar_1.SC_Door_Hangar_1" (`SceneComponent.K2_GetComponentLocation` (`self.Box`)) (struct) 0.2 0.9 0.0 "/Game/Audio/AttenuationVolume/AV_MonsterFootstep.AV_MonsterFootstep" null))
  (set `self.CloseSound` _returnvalue)
  (goto _label :!via `Reverse`))

(event `self.Box.OnComponentBeginOverlap`
  (params (OverlappedComponent :type "PrimitiveComponent Object Reference") (OtherActor :type "Actor Object Reference") (OtherComp :type "PrimitiveComponent Object Reference") (OtherBodyIndex :type Integer) (bFromSweep :type Boolean) (SweepResult :type "HitResult Structure (by ref)"))
  (cast `/Game/Blueprint/BP_FirstPersonCharacter` OtherActor)
  (`self.Open`))

(event `self.Box.OnComponentEndOverlap`
  (params (OverlappedComponent :type "PrimitiveComponent Object Reference") (OtherActor :type "Actor Object Reference") (OtherComp :type "PrimitiveComponent Object Reference") (OtherBodyIndex :type Integer))
  (cast `/Game/Blueprint/BP_FirstPersonCharacter` OtherActor)
  (`self.Close`))

(fn `UserConstructionScript`)