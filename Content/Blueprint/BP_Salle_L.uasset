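; BP_Salle_L is a room actor with fourteen child-actor lab doors, one designated as the exit by index.
; Its construction script orders the doors, stores the exit reference, applies two glyph sets to their decals, and removes, locks or makes each openable from a state array.
; At runtime, two box triggers pass the exit index to the zero-G player pawn and update its widget when that index differs.
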(event `self.ReceiveBeginPlay`)

(event `SetOut`
  (bind _asbp_zero_gpawn_cam (cast `/Game/Blueprint/BP_ZeroGPawnCam` (`GameplayStatics.GetPlayerPawn` 0)))
  (set `/Game/Blueprint/BP_ZeroGPawnCam.OutDoorInt` (`self.PorteOut`) _asbp_zero_gpawn_cam)
  (`/Game/UserInterface/WPB_HUDInGame.Set0GravityPorteOut` (`/Game/Blueprint/BP_ZeroGPawnCam.WidRef` _asbp_zero_gpawn_cam) false))

(event `self.Box.OnComponentBeginOverlap`
  (params (OverlappedComponent :type "PrimitiveComponent Object Reference") (OtherActor :type "Actor Object Reference") (OtherComp :type "PrimitiveComponent Object Reference") (OtherBodyIndex :type Integer) (bFromSweep :type Boolean) (SweepResult :type "HitResult Structure (by ref)"))
  (bind _asbp_zero_gpawn_cam (cast `/Game/Blueprint/BP_ZeroGPawnCam` OtherActor))
  (if (!= (`/Game/Blueprint/BP_ZeroGPawnCam.OutDoorInt` _asbp_zero_gpawn_cam) (`self.PorteOut`))
    (`self.SetOut`)))

(event `self.Box1.OnComponentBeginOverlap`
  (params (OverlappedComponent :type "PrimitiveComponent Object Reference") (OtherActor :type "Actor Object Reference") (OtherComp :type "PrimitiveComponent Object Reference") (OtherBodyIndex :type Integer) (bFromSweep :type Boolean) (SweepResult :type "HitResult Structure (by ref)"))
  (bind _asbp_zero_gpawn_cam (cast `/Game/Blueprint/BP_ZeroGPawnCam` OtherActor))
  (if (!= (`/Game/Blueprint/BP_ZeroGPawnCam.OutDoorInt` _asbp_zero_gpawn_cam) (`self.PorteOut`))
    (`self.SetOut`)))

(fn `UserConstructionScript`
  (`KismetArrayLibrary.Array_Clear` (`self.PorteChild`))
  (set `self.PorteChild` (`|MakeArray` (`self.Porte_Labs3`) (`self.Porte_Labs2`) (`self.Porte_Labs1`) (`self.Porte_Labs`) (`self.Porte_Labs8`) (`self.Porte_Labs9`) (`self.Porte_Labs7`) (`self.Porte_Labs4`) (`self.Porte_Labs5`) (`self.Porte_Labs6`) (`self.Porte_Labs13`) (`self.Porte_Labs12`) (`self.Porte_Labs11`) (`self.Porte_Labs10`)))
  (set `self.OutRef` (`|GetArrayItem` (`self.PorteChild`) (`self.PorteOut`)))
  (for (_array_element _array_index) (`self.Porte01Glyphe`)
    (bind _asporte_labs (cast `/Game/Blueprint/Porte_Labs` (`ChildActorComponent.ChildActor` (`|GetArrayItem` (`self.PorteChild`) _array_index))))
    (set `/Game/Blueprint/Porte_Labs.NumeroPorte01` _array_element _asporte_labs)
    (`/Game/Blueprint/Porte_Labs.SwitchDecal` _asporte_labs true))
  (for (_array_element_2 _array_index_2) (`self.Porte02Glyphe`)
    (bind _asporte_labs_2 (cast `/Game/Blueprint/Porte_Labs` (`ChildActorComponent.ChildActor` (`|GetArrayItem` (`self.PorteChild`) _array_index_2))))
    (set `/Game/Blueprint/Porte_Labs.NumeroPorte02` _array_element_2 _asporte_labs_2)
    (`/Game/Blueprint/Porte_Labs.SwitchDecal` _asporte_labs_2 false))
  (for (_array_element_3 _array_index_3) (`self.PorteState`)
    (if (`|EnumEquality` _array_element_3 "NewEnumerator1")
      (bind _output (`|GetArrayItem` (`self.PorteChild`) _array_index_3))
      (`ActorComponent.K2_DestroyComponent` _output)
      (elif (`|EnumEquality` _array_element_3 "NewEnumerator2")
        (bind _childactor (`ChildActorComponent.ChildActor` _output))
        (bind _asporte_labs_3 (cast `/Game/Blueprint/Porte_Labs` _childactor))
        (set `/Game/Blueprint/Porte_Labs.Openable?` false _asporte_labs_3)
        (else
          (bind _asporte_labs_4 (cast `/Game/Blueprint/Porte_Labs` _childactor))
          (set `/Game/Blueprint/Porte_Labs.Openable?` true _asporte_labs_4))))))