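; PATHPOINT is a path point actor that carries a teleport flag and a wait time, with editor-visible icons reflecting both settings.
; Its construction script gives TeleportState a nav-link sprite when IsTeleport is set and TimeState a chrono sprite when WaitTime is positive.
; Otherwise each falls back to the BlendFunc_DefBase sprite.
; The event graph has no active logic, so the Blueprint itself does no movement, teleporting or waiting.
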(fn `UserConstructionScript`
  (bind _teleportstate (`self.TeleportState`))
  (bind _timestate (`self.TimeState`))
  (if (`self.IsTeleport?`)
    (`BillboardComponent.SetSprite` _teleportstate "/Engine/EditorResources/AI/S_NavLink.S_NavLink")
    (else
      (`BillboardComponent.SetSprite` _teleportstate "/Engine/EngineMaterials/BlendFunc_DefBase.BlendFunc_DefBase")))
  (if (> (`self.WaitTime`) 0.0)
    (`BillboardComponent.SetSprite` _timestate "/Game/Textures/chrono.chrono")
    (else
      (`BillboardComponent.SetSprite` _timestate "/Engine/EngineMaterials/BlendFunc_DefBase.BlendFunc_DefBase"))))