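; BP_Body is the first-person player body, adding the Enhanced Input movement context on possession and handling move, look and interact.
; Interact line-traces from the camera with persistent debug drawing, messaging only BP_Lift2_Plateforme box hits through BPI_Interact.
; Overlapping another actor sends it a fixed ID via CheckIDMessage.
; The construction script adds, then immediately destroys, an AC_0X00A21E component; old axis events remain as empty stubs.
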(event `self.ReceivePossessed`
  (params (NewController :type "Controller Object Reference"))
  ;[1 0 0] Initializing Neural connections
  (bind _asplayer_controller (cast `PlayerController` NewController))
  (`EnhancedInputSubsystemInterface.AddMappingContext` (pcsubsystem `EnhancedInputLocalPlayerSubsystem` _asplayer_controller) "/Game/ScienceLab/IMC_Movement.IMC_Movement" 0 (struct)))

(event `EnhancedInput|/Game/ScienceLab/IA_Interact`
  (params (ActionValue :type Boolean) (ElapsedSeconds :type "Float (double-precision)") (TriggeredSeconds :type "Float (double-precision)") (InputAction :type "InputAction Object Reference" :default "/Game/ScienceLab/IA_Interact.IA_Interact"))
  (bind _firstpersoncamera (`self.FirstPersonCamera`))
  (bind _returnvalue (`SceneComponent.K2_GetComponentLocation` _firstpersoncamera))
  ;[0 0.3281 0] NeuralPsychicInteractionV2.0
  (:`Started`
    (bind _outhit (`KismetSystemLibrary.LineTraceSingle` :`Start` _returnvalue :`End` (+ (* (`SceneComponent.GetForwardVector` _firstpersoncamera) 500.0) _returnvalue) :`TraceChannel` "TraceTypeQuery1" :`DrawDebugType` "Persistent"))
    (bind _asbox_collision (cast `BoxComponent` (`.HitComponent` (`GameplayStatics.BreakHitResult` _outhit))))
    (bind _asbp_lift_2_plateforme (cast `/Game/Blueprint/BP_Lift2_Plateforme` (`ActorComponent.GetOwner` _asbox_collision)))
    (if (`KismetSystemLibrary.DoesImplementInterface` _asbp_lift_2_plateforme "/Game/Blueprint/BPI_Interact.BPI_Interact_C")
      (message `/Game/Blueprint/BPI_Interact.Interact` _asbp_lift_2_plateforme))))

(event `InputAxis|MoveForward` :consume false :overrideparent false
  (params (AxisValue :type "Float (single-precision)"))
  ;[0 0.3281 0] OLD
)

(event `EnhancedInput|/Game/ScienceLab/IA_Move`
  (params (ActionValue :type "Vector2D Structure") (ElapsedSeconds :type "Float (double-precision)") (TriggeredSeconds :type "Float (double-precision)") (InputAction :type "InputAction Object Reference" :default "/Game/ScienceLab/IA_Move.IA_Move"))
  ;[0.006671 0.151 0] Controls
  (:`Triggered`
    (`self.AddMovementInput` (+ (* ActionValue_X (`self.GetActorForwardVector`)) (* ActionValue_Y (`self.GetActorRightVector`))))))

(event `InputAxis|MoveRight` :consume false :overrideparent false
  (params (AxisValue :type "Float (single-precision)"))
  ;[0 0.3281 0] OLD
)

(event `InputAxis|Turn` :overrideparent false
  (params (AxisValue :type "Float (single-precision)"))
  ;[0 0.3281 0] OLD
)

(event `EnhancedInput|/Game/ScienceLab/IA_Turn`
  (params (ActionValue :type "Vector2D Structure") (ElapsedSeconds :type "Float (double-precision)") (TriggeredSeconds :type "Float (double-precision)") (InputAction :type "InputAction Object Reference" :default "/Game/ScienceLab/IA_Turn.IA_Turn"))
  ;[0.006671 0.151 0] HeadRotation
  (:`Triggered`
    (`self.AddControllerYawInput` ActionValue_X)
    (`self.AddControllerPitchInput` ActionValue_Y)))

(event `InputAxis|LookUp` :overrideparent false
  (params (AxisValue :type "Float (single-precision)"))
  ;[0 0.3281 0] OLD
)

(event `self.ReceiveActorBeginOverlap`
  (params (OtherActor :type "Actor Object Reference"))
  ;[1 0 0] ID
  (message `/Game/Blueprint/BPI_Identity.CheckID` OtherActor "id_29"))

(fn `UserConstructionScript`
  (`|ExecutionSequence`
    (:`then_0`
      (`AddComponent|NODE_AddAC_0X00A21E-0`))
    (:`then_1`
      ;[0 0.3281 0] RAM
      (`ActorComponent.K2_DestroyComponent` (`self.GetComponentByClass` "/Game/Blueprint/AC_0X00A21E.AC_0X00A21E_C")))))