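; BP_VerticalDoor is a door that slides vertically, toggling between open and closed on each Open/Close call.
; After a caller-supplied delay, it starts one of two sparkle effects at random, and a FlipFlop plays or reverses a Timeline.
; The Timeline lerps the door's relative Z between a fixed height and OpenOffset, then stops both effects when finished.
; The WiredAction event is empty.
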(event `Open/Close`
  (params (Delay :type "Float (double-precision)"))
  (`KismetSystemLibrary.Delay` Delay)
  (`NiagaraComponent.SetVariableFloat` (select `bool` (`KismetMathLibrary.RandomBool`) :`false` (`self.NS_doorsparkles1`) :`true` (`self.NS_doorsparkles`)) "spawnrate" 60.0)
  (`/Engine/EditorBlueprintResources/StandardMacros.FlipFlop`
    (:`A`
      (bind (_direction _alpha) (`Timeline|Timeline_0` :!label _label)
        (:`Update`
          (`SceneComponent.K2_SetRelativeLocation` (`self.Door`) (`KismetMathLibrary.VLerp` (0.0 0.0 270.0) (`KismetMathLibrary.MakeVector` 0.0 0.0 (`self.OpenOffset`)) _alpha) false false))
        (:`Finished`
          (`NiagaraComponent.SetVariableFloat` (`self.NS_doorsparkles1`) "spawnrate" 0.0)
          (`NiagaraComponent.SetVariableFloat` (`self.NS_doorsparkles`) "spawnrate" 0.0))))
    (:`B`
      (goto _label :!via `Reverse`))))

(event `/Game/Blueprint/BPI_WiredActor.WiredAction`)

(fn `UserConstructionScript`)