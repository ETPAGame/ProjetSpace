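; Checkpoint actor that respawns a pawn at its own location and is linked to a set of wired light actors.
; RESPAWN teleports the pawn and sends a reset message to each linked actor implementing BPI_WiredActor.
; WiredAction calls BreakLoop on the player controller with an index chosen by actor tag, then destroys the checkpoint.
; The construction script draws a spline from each linked actor to the checkpoint to visualise the wiring.
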(event `RESPAWN`
  (params (pawn :type "Pawn Object Reference"))
  (`self.K2_TeleportTo` :`self` pawn :`DestLocation` (`self.K2_GetActorLocation`))
  (for _array_element (`self.WiredLight`)
    (if (`KismetSystemLibrary.DoesImplementInterface` _array_element "/Game/Blueprint/BPI_WiredActor.BPI_WiredActor_C")
      (message `/Game/Blueprint/BPI_WiredActor.ResetActor` _array_element))))

(event `/Game/Blueprint/BPI_WiredActor.WiredAction`
  (bind _asbp_player_controller (cast `/Game/Blueprint/BP_PlayerController` (`GameplayStatics.GetPlayerController` 0)))
  (`/Game/Blueprint/BP_PlayerController.BreakLoop` _asbp_player_controller (`KismetMathLibrary.SelectInt` 1 2 (`self.ActorHasTag` "1")))
  (`self.K2_DestroyActor`))

(fn `UserConstructionScript`
  ;[1 0.5141 0.9922] Draw Link
  (for _array_element (`self.WiredLight`)
    (`/Engine/EditorBlueprintResources/StandardMacros.IsValid` _array_element
      (:`Is Valid`
        (bind _returnvalue (`AddComponent|NODE_AddSplineComponent-0`))
        (`SplineComponent.SetSplinePoints` _returnvalue (`|MakeArray` (`self.K2_GetActorLocation` _array_element) (`SceneComponent.K2_GetComponentLocation` (`self.1`))) "World" true)))))