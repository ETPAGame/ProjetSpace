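; Switchable rect light fixture that toggles on and off when its WiredAction event fires.
; A FlipFlop runs the Light timeline forward or back to fade intensity between full and Offvalue, while swapping the color on a dynamic unlit material for the mesh's emissive slot.
; The construction script fits source size and attenuation radius to the actor's scale and applies Offvalue intensity when TurnOff is set.
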(event `/Game/Blueprint/BPI_WiredActor.WiredAction`
  (`self.Switch Light`))

(event `Switch Light`
  (`/Engine/EditorBlueprintResources/StandardMacros.FlipFlop`
    (:`A`
      (`MaterialInstanceDynamic.SetVectorParameterValue` (`self.emisiveMAT`) "color" (make `LinearColor` 1.0 1.0 1.0 1.0))
      (bind (_direction _alpha) (`Timeline|Light` :!via `Reverse` :!label _label)
        (:`Update`
          (`LightComponent.SetIntensity` (`self.RectLight`) (`KismetMathLibrary.Lerp` 40000.0 (`self.offvalue`) _alpha)))))
    (:`B`
      (`MaterialInstanceDynamic.SetVectorParameterValue` (`self.emisiveMAT`) "color" (make `LinearColor` 0.0))
      (goto _label))))

(event `self.ReceiveBeginPlay`
  (bind _returnvalue (`KismetMaterialLibrary.CreateDynamicMaterialInstance` "/Game/Material/M_lightUnlit.M_lightUnlit"))
  (bind _output_get (set `self.emisiveMAT` _returnvalue))
  (`PrimitiveComponent.SetMaterial` (`self.StaticMesh`) 1 _output_get))

(fn `UserConstructionScript`
  (bind _rectlight (`self.RectLight`))
  (bind (_returnvalue_x _returnvalue_y) (`KismetMathLibrary.BreakVector` (`SceneComponent.K2_GetComponentScale` (`self.DefaultSceneRoot`))))
  (`RectLightComponent.SetSourceWidth` _rectlight (* (`RectLightComponent.SourceWidth` _rectlight) _returnvalue_y))
  (`RectLightComponent.SetSourceHeight` _rectlight (* (`RectLightComponent.SourceHeight` _rectlight) _returnvalue_x))
  (`LocalLightComponent.SetAttenuationRadius` (`self.RectLight`) (* _returnvalue_y 1000.0))
  (if (`self.turnOff`)
    (`LightComponent.SetIntensity` (`self.RectLight`) (`self.offvalue`))))