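; Lockable sliding double door that opens on box overlap by the player, zero-G pawn, monster or cine camera.
; A timeline slides both halves; exit closes them, except for cameras, and locked doors play a delayed denial sound if the player remains.
; WiredAction toggles the lock, may open or close the door, and swaps red/green frame materials and lights.
; Construction script previews lock and open state; ResetActor restores settings cached at BeginPlay.
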(event `/Game/Blueprint/BPI_WiredActor.WiredAction`
  (`self.Switch`)
  (set `self.Locked?` (not (`self.Locked?`)))
  (if (not (not (`self.CloseOnLock`)))
    (`self.Close`))
  (if (`PrimitiveComponent.IsOverlappingActor` (`self.Box`) (`GameplayStatics.GetPlayerCharacter` 0))
    (`self.Open`))
  (if (`self.StartOpen?`)
    (`self.Close`)))

(event `self.Box.OnComponentBeginOverlap`
  (params (OverlappedComponent :type "PrimitiveComponent Object Reference") (OtherActor :type "Actor Object Reference") (OtherComp :type "PrimitiveComponent Object Reference") (OtherBodyIndex :type Integer) (bFromSweep :type Boolean) (SweepResult :type "HitResult Structure (by ref)"))
  (cast `CineCameraActor` OtherActor
    (:`then`
      _)
    (:`CastFailed`
      (cast `/Game/Blueprint/BP_FirstPersonCharacter` OtherActor
        (:`then`
          _)
        (:`CastFailed`
          (cast `/Game/Blueprint/BP_ZeroGPawnCam` OtherActor
            (:`then`
              _)
            (:`CastFailed`
              (cast `/Game/Monster/BP_Monster` OtherActor)))))))
  (if (not (`self.Locked?`))
    (`self.Open`)
    (else
      (`KismetSystemLibrary.RetriggerableDelay` 2.5)
      (if (`PrimitiveComponent.IsOverlappingActor` (`self.Box`) (`GameplayStatics.GetPlayerCharacter` 0))
        (`GameplayStatics.PlaySoundAtLocation` "/Game/Audio/SFX/Environment/Door/SC_Negative_Door.SC_Negative_Door" (`SceneComponent.K2_GetComponentLocation` (`self.DefaultSceneRoot`)) (struct) 1.0 1.0 0.0 null null null null)))))

(event `Switch`
  (bind _sm_doorway_small_a1 (`self.SM_Doorway_Small_A1`))
  (bind _sm_doorway_small_a (`self.SM_Doorway_Small_A`))
  (if (`self.Locked?`)
    (`/Engine/EditorBlueprintResources/StandardMacros.FlipFlop`
      (:`A`
        (`PrimitiveComponent.SetMaterial` _sm_doorway_small_a1 1 "/Game/Material/M_TEMP_GreenEmissive.M_TEMP_GreenEmissive")
        (`PrimitiveComponent.SetMaterial` _sm_doorway_small_a 1 "/Game/Material/M_TEMP_GreenEmissive.M_TEMP_GreenEmissive")
        (set `self.Color` (struct :`R` 0.321186 :`G` 1.0 :`A` 1.0) :!label _label))
      (:`B`
        (`PrimitiveComponent.SetMaterial` _sm_doorway_small_a1 1 "/Game/Material/M_TEMP_RedEmissive.M_TEMP_RedEmissive")
        (`PrimitiveComponent.SetMaterial` _sm_doorway_small_a 1 "/Game/Material/M_TEMP_RedEmissive.M_TEMP_RedEmissive")
        (set `self.Color` (struct :`R` 1.0 :`B` 0.046545 :`A` 1.0) :!label _label_2)))
    (else
      (`/Engine/EditorBlueprintResources/StandardMacros.FlipFlop`
        (:`A`
          (`PrimitiveComponent.SetMaterial` _sm_doorway_small_a 1 "/Game/Material/M_TEMP_RedEmissive.M_TEMP_RedEmissive")
          (`PrimitiveComponent.SetMaterial` _sm_doorway_small_a1 1 "/Game/Material/M_TEMP_RedEmissive.M_TEMP_RedEmissive")
          (goto _label_2))
        (:`B`
          (`PrimitiveComponent.SetMaterial` _sm_doorway_small_a 1 "/Game/Material/M_TEMP_GreenEmissive.M_TEMP_GreenEmissive")
          (`PrimitiveComponent.SetMaterial` _sm_doorway_small_a1 1 "/Game/Material/M_TEMP_GreenEmissive.M_TEMP_GreenEmissive")
          (goto _label)))))
  (`self.Set LightColor` (`self.Color`)))

(event `self.Box.OnComponentEndOverlap`
  (params (OverlappedComponent :type "PrimitiveComponent Object Reference") (OtherActor :type "Actor Object Reference") (OtherComp :type "PrimitiveComponent Object Reference") (OtherBodyIndex :type Integer))
  (cast `/Game/Blueprint/BP_FirstPersonCharacter` OtherActor
    (:`then`
      _)
    (:`CastFailed`
      (cast `/Game/Blueprint/BP_ZeroGPawnCam` OtherActor
        (:`then`
          _)
        (:`CastFailed`
          (cast `/Game/Monster/BP_Monster` OtherActor)))))
  (if (not (`self.Locked?`))
    (`self.Close`)))

(event `Open`
  (`GameplayStatics.PlaySoundAtLocation` "/Game/Audio/SFX/Environment/Door/SC_DoubleDoor.SC_DoubleDoor" (`SceneComponent.K2_GetComponentLocation` (`self.Box`)) (struct) 1.0 1.1 0.0 null null null null)
  (bind (_direction _alpha) (`Timeline|DoorsTimeline` :!label _label_3)
    (:`Update`
      (bind _returnvalue (`KismetMathLibrary.VLerp` (0.0 80.0 0.0) (`KismetMathLibrary.MakeVector` 0.0 (`self.OpenDestination`)) _alpha))
      (`SceneComponent.K2_SetRelativeLocation` (`self.DoorR`) _returnvalue false false)
      (`SceneComponent.K2_SetRelativeLocation` (`self.DoorL`) (`KismetMathLibrary.NegateVector` _returnvalue) false false))))

(event `/Game/Blueprint/BPI_WiredActor.ResetActor`
  (bind _locked_ (`self.Locked?`))
  (set `self.OpenDestination` (`self.Open DestinationReset`))
  (bind _output_get (set `self.Locked?` (`self.Locked?Reset`)))
  (if _output_get
    (`PrimitiveComponent.SetMaterial` (`self.SM_Doorway_Small_A`) 1 "/Game/Material/M_TEMP_RedEmissive.M_TEMP_RedEmissive")
    (`PrimitiveComponent.SetMaterial` (`self.SM_Doorway_Small_A1`) 1 "/Game/Material/M_TEMP_RedEmissive.M_TEMP_RedEmissive"))
  (bind _output_get_2 (set `self.StartOpen?` (`self.Start Open?Reset`)))
  (if _output_get_2
    (`self.Open`)
    (else
      (`self.Close`)))
  (set `self.CloseOnLock` (`self.Close on LockReset`))
  (`PrimitiveComponent.SetMaterial` (`self.SM_Doorway_Small_A1`) 1 (select `bool` _locked_ :`false` "/Game/Material/M_TEMP_GreenEmissive.M_TEMP_GreenEmissive" :`true` "/Game/Material/M_TEMP_RedEmissive.M_TEMP_RedEmissive" :!type "MaterialInterface Object Reference"))
  (`PrimitiveComponent.SetMaterial` (`self.SM_Doorway_Small_A`) 1 (select `bool` _locked_ :`false` "/Game/Material/M_TEMP_GreenEmissive.M_TEMP_GreenEmissive" :`true` "/Game/Material/M_TEMP_RedEmissive.M_TEMP_RedEmissive" :!type "MaterialInterface Object Reference"))
  (`self.Set LightColor` (select `bool` _locked_ :`false` (struct :`R` 0.099748 :`G` 1.0 :`A` 1.0) :`true` (struct :`R` 1.0 :`B` 0.054287 :`A` 1.0) :!type "LinearColor Structure")))

(event `Close`
  (goto _label_3 :!via `Reverse`))

(event `self.ReceiveBeginPlay`
  (set `self.Open DestinationReset` (`self.OpenDestination`))
  (set `self.Locked?Reset` (`self.Locked?`))
  (set `self.Start Open?Reset` (`self.StartOpen?`))
  (set `self.Reset` (`self.Color`))
  (set `self.Close on LockReset` (`self.CloseOnLock`)))

(fn `Set LightColor`
  (params (Color :type "LinearColor Structure"))
  (`LightComponent.SetLightColor` (`self.PointLight1`) Color true)
  (`LightComponent.SetLightColor` (`self.PointLight`) Color true))

(fn `UserConstructionScript`
  (bind _locked_ (`self.Locked?`))
  (bind _returnvalue (`KismetMathLibrary.MakeVector` 0.0 (`self.OpenDestination`)))
  (`PrimitiveComponent.SetMaterial` (`self.SM_Doorway_Small_A1`) 1 (select `bool` _locked_ :`false` "/Game/Material/M_TEMP_GreenEmissive.M_TEMP_GreenEmissive" :`true` "/Game/Material/M_TEMP_RedEmissive.M_TEMP_RedEmissive" :!type "MaterialInterface Object Reference"))
  (`PrimitiveComponent.SetMaterial` (`self.SM_Doorway_Small_A`) 1 (select `bool` _locked_ :`false` "/Game/Material/M_TEMP_GreenEmissive.M_TEMP_GreenEmissive" :`true` "/Game/Material/M_TEMP_RedEmissive.M_TEMP_RedEmissive" :!type "MaterialInterface Object Reference"))
  (`self.Set LightColor` (select `bool` _locked_ :`false` (struct :`R` 0.099748 :`G` 1.0 :`A` 1.0) :`true` (struct :`R` 1.0 :`B` 0.054287 :`A` 1.0) :!type "LinearColor Structure"))
  (if (`self.StartOpen?`)
    (`SceneComponent.K2_SetRelativeLocation` (`self.DoorR`) _returnvalue false false)
    (`SceneComponent.K2_SetRelativeLocation` (`self.DoorL`) (`KismetMathLibrary.NegateVector` _returnvalue) false false)))