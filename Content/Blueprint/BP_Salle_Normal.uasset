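; Standard room Blueprint with six child-actor doors, one marked as the exit by index.
; The construction script randomly flips and rotates PROJOS, assigns each door's glyph decals, and removes, locks or unlocks doors by state.
; When the zero-G pawn enters with a different exit index, the room passes it its own, updates the HUD and starts timeline Aaa at random speed.
; Leaving stops the timeline only if the indices differ.
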(event `SetOut`
  (bind _asbp_zero_gpawn_cam (cast `/Game/Blueprint/BP_ZeroGPawnCam` (`GameplayStatics.GetPlayerPawn` 0)))
  (set `/Game/Blueprint/BP_ZeroGPawnCam.OutDoorInt` (`self.PorteOut`) _asbp_zero_gpawn_cam)
  (bind _asbp_player_controller (cast `/Game/Blueprint/BP_PlayerController` (`GameplayStatics.GetPlayerController` 0)))
  (`/Game/UserInterface/WPB_HUDInGame.Set0GravityPorteOut` (`/Game/Blueprint/BP_PlayerController.HUDRef` _asbp_player_controller) false))

(event `self.Box.OnComponentBeginOverlap`
  (params (OverlappedComponent :type "PrimitiveComponent Object Reference") (OtherActor :type "Actor Object Reference") (OtherComp :type "PrimitiveComponent Object Reference") (OtherBodyIndex :type Integer) (bFromSweep :type Boolean) (SweepResult :type "HitResult Structure (by ref)"))
  (bind _asbp_zero_gpawn_cam (cast `/Game/Blueprint/BP_ZeroGPawnCam` OtherActor))
  (if (!= (`/Game/Blueprint/BP_ZeroGPawnCam.OutDoorInt` _asbp_zero_gpawn_cam) (`self.PorteOut`))
    (`self.SetOut`)
    (`self.startDelay`)))

(event `startDelay`
  (`TimelineComponent.SetPlayRate` (`self.aaa`) (`KismetMathLibrary.RandomFloatInRange` 0.8 1.2))
  (`Timeline|aaa` :!via `PlayFromStart` :!label _label))

(event `StopDelay`
  (goto _label :!via `Stop`))

(event `self.Box.OnComponentEndOverlap`
  (params (OverlappedComponent :type "PrimitiveComponent Object Reference") (OtherActor :type "Actor Object Reference") (OtherComp :type "PrimitiveComponent Object Reference") (OtherBodyIndex :type Integer))
  (bind _asbp_zero_gpawn_cam (cast `/Game/Blueprint/BP_ZeroGPawnCam` OtherActor))
  (if (!= (`/Game/Blueprint/BP_ZeroGPawnCam.OutDoorInt` _asbp_zero_gpawn_cam) (`self.PorteOut`))
    (`self.StopDelay`)))

(fn `UserConstructionScript`
  (bind _projos (`self.PROJOS`))
  (`SceneComponent.SetRelativeScale3D` _projos (`KismetMathLibrary.MakeVector` 1.0 1.0 (`KismetMathLibrary.Conv_IntToDouble` (select `bool` (`KismetMathLibrary.RandomBool`) :`false` -1 :`true` 1))))
  (`SceneComponent.K2_SetRelativeRotation` _projos (`KismetMathLibrary.MakeRotator` 0.0 0.0 (select `int` (`KismetMathLibrary.RandomIntegerInRange` 0 3) :`0` 0.0 :`1` 90.0 :`2` 180.0 :`3` -90.0)) false false)
  (`KismetArrayLibrary.Array_Clear` (`self.PorteChild`))
  (set `self.PorteChild` (`|MakeArray` (`self.Porte_Labs`) (`self.Porte_Labs3`) (`self.Porte_Labs1`) (`self.Porte_Labs2`) (`self.Porte_Labs4`) (`self.Porte_Labs5`)))
  (set `self.OutRef` (`|GetArrayItem` (`self.PorteChild`) (`self.PorteOut`)))
  (for (_array_element _array_index) (`self.Porte01Glyphe`)
    (bind _asporte_labs (cast `/Game/Blueprint/Porte_Labs` (`ChildActorComponent.ChildActor` (`|GetArrayItem` (`self.PorteChild`) _array_index))))
    (set `/Game/Blueprint/Porte_Labs.NumeroPorte01` _array_element _asporte_labs)
    (`/Game/Blueprint/Porte_Labs.SwitchDecal` _asporte_labs true))
  (for (_array_element_2 _array_index_2) (`self.Porte02Glyphe`)
    (bind _asporte_labs_2 (cast `/Game/Blueprint/Porte_Labs` (`ChildActorComponent.ChildActor` (`|GetArrayItem` (`self.PorteChild`) _array_index_2))))
    (set `/Game/Blueprint/Porte_Labs.NumeroPorte02` _array_element_2 _asporte_labs_2)
    (`/Game/Blueprint/Porte_Labs.SwitchDecal` _asporte_labs_2 false))
  (for (_array_element_3 _array_index_3) (`self.PorteState`)
    (if (`|EnumEquality` _array_element_3 "NewEnumerator1")
      (bind _output (`|GetArrayItem` (`self.PorteChild`) _array_index_3))
      (`ActorComponent.K2_DestroyComponent` _output)
      (elif (`|EnumEquality` _array_element_3 "NewEnumerator2")
        (bind _childactor (`ChildActorComponent.ChildActor` _output))
        (bind _asporte_labs_3 (cast `/Game/Blueprint/Porte_Labs` _childactor))
        (set `/Game/Blueprint/Porte_Labs.Openable?` false _asporte_labs_3)
        (else
          (bind _asporte_labs_4 (cast `/Game/Blueprint/Porte_Labs` _childactor))
          (set `/Game/Blueprint/Porte_Labs.Openable?` true _asporte_labs_4))))))