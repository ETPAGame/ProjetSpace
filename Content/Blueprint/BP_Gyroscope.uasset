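; BP_Gyroscope is a sphere indicator meant to visualize a zero-G pawn's velocity through directional materials.
; Its construction script creates six dynamic material instances on the sphere, named in French for south, north, west, east, far and near.
; A fast looping timer polls the referenced pawn, mapping positive X velocity to the east material's Amount parameter.
; Y and Z checks are empty, and the other five materials are never updated.
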(event `self.ReceiveBeginPlay`
  (`KismetSystemLibrary.K2_SetTimerDelegate` (delegate `CustomEvent_0`) 0.02 true))

(event `CustomEvent_0`
  (bind _returnvalue (`self.GetVelocity` (`self.ZeroGPawn Ref`)))
  (`/Engine/EditorBlueprintResources/StandardMacros.IsValid` (`self.ZeroGPawn Ref`)
    (:`Is Valid`
      (`|ExecutionSequence`
        (:`then_0`
          (if (> (.x _returnvalue) 0.0)
            (`MaterialInstanceDynamic.SetScalarParameterValue` (`self.Est`) "Amount" (`KismetMathLibrary.MapRangeClamped` (.x _returnvalue) 0.0 600.0 20.0))))
        (:`then_1`
          (if (> (.y _returnvalue) 0.0)
            _))
        (:`then_2`
          (if (> (.z _returnvalue) 0.0)
            _))))))

(fn `UserConstructionScript`
  (bind _returnvalue (`PrimitiveComponent.CreateDynamicMaterialInstance` (`self.Sphere`) 0 null "None"))
  (set `self.Sud` _returnvalue)
  (bind _returnvalue_2 (`PrimitiveComponent.CreateDynamicMaterialInstance` (`self.Sphere`) 1 null "None"))
  (set `self.Nord` _returnvalue_2)
  (bind _returnvalue_3 (`PrimitiveComponent.CreateDynamicMaterialInstance` (`self.Sphere`) 2 null "None"))
  (set `self.Ouest` _returnvalue_3)
  (bind _returnvalue_4 (`PrimitiveComponent.CreateDynamicMaterialInstance` (`self.Sphere`) 3 null "None"))
  (set `self.Est` _returnvalue_4)
  (bind _returnvalue_5 (`PrimitiveComponent.CreateDynamicMaterialInstance` (`self.Sphere`) 4 null "None"))
  (set `self.Loin` _returnvalue_5)
  (bind _returnvalue_6 (`PrimitiveComponent.CreateDynamicMaterialInstance` (`self.Sphere`) 5 null "None"))
  (set `self.Pres` _returnvalue_6))