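; BP_SAS_Transition is an airlock (SAS) that moves the player to another location behind sliding doors.
; When ToGo is set, box overlap switches lights, closes the door and, after a delay, teleports the first-person or zero-G pawn to WhereToGo with yaw flipped 180°.
; It then calls the destination's OpenDoor and triggers TriggerEnd, WallManager and WarningManager.
; Timelines slide each door mesh pair, and the first-person character's LightGesture follows box overlap.
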(event `OpenDoor`
  (bind _staticmesh6 (`self.StaticMesh6`))
  (bind _staticmesh7 (`self.StaticMesh7`))
  (`KismetSystemLibrary.Delay` 0.7)
  (bind _output_get (set `self.Relative Location2` (`SceneComponent.RelativeLocation` _staticmesh6)))
  (bind _output_get_2 (set `self.Relative Location1` (`SceneComponent.RelativeLocation` _staticmesh7)))
  (bind (_direction _newtrack_0) (`Timeline|OpenLerp`)
    (:`Update`
      (bind (_x _y _z) (`KismetMathLibrary.BreakVector3f` _output_get))
      (`SceneComponent.K2_SetRelativeLocation` _staticmesh6 (`KismetMathLibrary.MakeVector` _x (`KismetMathLibrary.Lerp` 81.98 151.93 _newtrack_0) _z) false false)
      (bind (_x_2 _y_2 _z_2) (`KismetMathLibrary.BreakVector3f` _output_get_2))
      (`SceneComponent.K2_SetRelativeLocation` _staticmesh7 (`KismetMathLibrary.MakeVector` _x_2 (`KismetMathLibrary.Lerp` -80.0 -166.2 _newtrack_0) _z_2) false false))))

(event `Close door`
  (bind _staticmesh5 (`self.StaticMesh5`))
  (bind _staticmesh4 (`self.StaticMesh4`))
  (bind _relativelocation (`SceneComponent.RelativeLocation` _staticmesh4))
  (bind _relativelocation_2 (`SceneComponent.RelativeLocation` _staticmesh5))
  (bind (_x _y _z) (`KismetMathLibrary.BreakVector3f` _relativelocation_2))
  (bind (_x_2 _y_2 _z_2) (`KismetMathLibrary.BreakVector3f` _relativelocation))
  (set `self.Relative Location2` _relativelocation_2)
  (set `self.Relative Location1` _relativelocation)
  (bind (_direction _newtrack_0) (`Timeline|CloseLerp`)
    (:`Update`
      (`SceneComponent.K2_SetRelativeLocation` _staticmesh5 (`KismetMathLibrary.MakeVector` _x (`KismetMathLibrary.Lerp` -144.86 -77.1 _newtrack_0) _z) false false)
      (`SceneComponent.K2_SetRelativeLocation` _staticmesh4 (`KismetMathLibrary.MakeVector` _x_2 (`KismetMathLibrary.Lerp` 159.21 80.74 _newtrack_0) _z_2) false false))))

(event `self.Box.OnComponentBeginOverlap`
  (params (OverlappedComponent :type "PrimitiveComponent Object Reference") (OtherActor :type "Actor Object Reference") (OtherComp :type "PrimitiveComponent Object Reference") (OtherBodyIndex :type Integer) (bFromSweep :type Boolean) (SweepResult :type "HitResult Structure (by ref)"))
  (bind _returnvalue (`GameplayStatics.GetPlayerController` 0))
  (bind (_returnvalue_roll _returnvalue_pitch _returnvalue_yaw) (`KismetMathLibrary.BreakRotator` (`Controller.GetControlRotation` _returnvalue)))
  (if (`self.ToGo?`)
    (for _array_element (`self.Light`)
      (set `/Game/Blueprint/BP_FlickeringLight_2.ForceStop?` true _array_element)
      (`/Game/Blueprint/BP_FlickeringLight_2.Switch` _array_element))
    (`self.Close door`)
    (bind _asbp_first_person_character (cast `/Game/Blueprint/BP_FirstPersonCharacter` OtherActor)
      (:`then`
        (`/Game/Blueprint/BP_FirstPersonCharacter.LightGesture` _asbp_first_person_character true))
      (:`CastFailed`
        (cast `/Game/Blueprint/BP_ZeroGPawnCam` OtherActor)))
    (`KismetSystemLibrary.Delay` (`self.DurationToGo`))
    (`self.K2_SetActorLocation` OtherActor (+ (`self.K2_GetActorLocation` (`self.WhereToGo`)) (0.0 0.0 86.0)) false false)
    (`Controller.SetControlRotation` _returnvalue (`KismetMathLibrary.MakeRotator` _returnvalue_roll _returnvalue_pitch (+ _returnvalue_yaw 180.0)))
    (`self.OpenDoor` (`self.WhereToGo`))
    (set `/Game/Blueprint/BP_triggerend.Activ?` true (`self.TriggerEnd`))
    (`/Game/Blueprint/BP_WallEmissiveManager.Eteindre` (`self.WallManager`))
    (`/Game/Blueprint/BP_EvacuationManager.WARNING` (`self.WarningManager`))))

(event `self.Box.OnComponentEndOverlap`
  (params (OverlappedComponent :type "PrimitiveComponent Object Reference") (OtherActor :type "Actor Object Reference") (OtherComp :type "PrimitiveComponent Object Reference") (OtherBodyIndex :type Integer))
  (bind _asbp_first_person_character (cast `/Game/Blueprint/BP_FirstPersonCharacter` OtherActor))
  (`/Game/Blueprint/BP_FirstPersonCharacter.LightGesture` _asbp_first_person_character false))

(fn `UserConstructionScript`)