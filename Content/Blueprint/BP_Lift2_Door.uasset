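; BP_Lift2_Door is a double swing door for a lift, opened by a BP_Body entering its collision volume.
; If PlatformIsOk, overlap opens the door and the referenced platform's door; otherwise it calls the platform, passing itself.
; Leaving closes the door, plus the platform's when PlatformIsOk.
; A timeline drives mirrored yaw on both leaves, played forward or reversed, and the construction script applies DoorPosition.
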(event `OpenDoor`
  (bind _doorposition (`self.DoorPosition`))
  (bind (_direction _newtrack_0) (`Timeline|Timeline_0` :!label _label)
    (:`Update`
      (set `self.DoorPosition` (`KismetMathLibrary.Lerp` 0.0 27.0 _newtrack_0))
      (`SceneComponent.K2_SetRelativeRotation` (`self.Lift02Door02`) (`KismetMathLibrary.MakeRotator` 0.0 0.0 _doorposition) false false)
      (`SceneComponent.K2_SetRelativeRotation` (`self.Lift02Door01`) (`KismetMathLibrary.MakeRotator` 0.0 0.0 (* _doorposition -1.0)) false false))))

(event `CloseDoor`
  (goto _label :!via `Reverse`))

(event `self.Collision.OnComponentBeginOverlap`
  (params (OverlappedComponent :type "PrimitiveComponent Object Reference") (OtherActor :type "Actor Object Reference") (OtherComp :type "PrimitiveComponent Object Reference") (OtherBodyIndex :type Integer) (bFromSweep :type Boolean) (SweepResult :type "HitResult Structure (by ref)"))
  (cast `/Game/Blueprint/BP_Body` OtherActor)
  (if (`self.PlatformIsOk?`)
    (`self.OpenDoor`)
    (`/Game/Blueprint/BP_Lift2_Plateforme.OpenDoor` (`self.PlatformRef`))
    (else
      (`/Game/Blueprint/BP_Lift2_Plateforme.CallPlateform` (`self.PlatformRef`) self))))

(event `self.Collision.OnComponentEndOverlap`
  (params (OverlappedComponent :type "PrimitiveComponent Object Reference") (OtherActor :type "Actor Object Reference") (OtherComp :type "PrimitiveComponent Object Reference") (OtherBodyIndex :type Integer))
  (cast `/Game/Blueprint/BP_Body` OtherActor)
  (`self.CloseDoor`)
  (if (`self.PlatformIsOk?`)
    (`/Game/Blueprint/BP_Lift2_Plateforme.CloseDoor` (`self.PlatformRef`) false)))

(fn `UserConstructionScript`
  (bind _doorposition (`self.DoorPosition`))
  ;[1 1 1] Movement
  (`SceneComponent.K2_SetRelativeRotation` (`self.Lift02Door02`) (`KismetMathLibrary.MakeRotator` 0.0 0.0 _doorposition) false false)
  (`SceneComponent.K2_SetRelativeRotation` (`self.Lift02Door01`) (`KismetMathLibrary.MakeRotator` 0.0 0.0 (* _doorposition -1.0)) false false))