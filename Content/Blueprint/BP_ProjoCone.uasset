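; BP_ProjoCone is a switchable projector spotlight that flickers at random intervals with sound.
; A self-rescheduling timer alternately plays and reverses a timeline, whose updates apply noisy sine-modulated intensity before settling at the default on finish.
; SetAllIntensity drives both the spotlight and the mesh material's "emi" parameter, keeping glow matched to light.
; Switch alternates between starting the flicker and forcing the light dark, using ForceStop to gate updates.
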(event `self.ReceiveBeginPlay`
  (`LightComponent.SetIntensity` (`self.SpotLight`) 0.0)
  (set `self.material` (`PrimitiveComponent.GetMaterial` (`self.projo`) 0))
  (`self.Start Flicker Loop`))

(event `Switch`
  ;[1 1 1] Switch Mode
  (`/Engine/EditorBlueprintResources/StandardMacros.FlipFlop`
    (:`A`
      (set `self.Force Stop?` false)
      (`self.Flicker`))
    (:`B`
      (set `self.Force Stop?` true)
      (`self.Set All Intensity` 0.0)
      (`self.break`))))

(event `Flicker`
  (bind _returnvalue (`KismetMathLibrary.RandomFloatInRange` 0.95 1.05))
  (bind _returnvalue_2 (`SceneComponent.K2_GetComponentLocation` (`self.projo`)))
  ;[1 1 1] Flicker
  (if (not (`self.Force Stop?`))
    (`/Engine/EditorBlueprintResources/StandardMacros.FlipFlop`
      (:`A`
        (`KismetSystemLibrary.Delay` (`KismetMathLibrary.RandomFloatInRange` 0.0 2.0))
        (`GameplayStatics.PlaySoundAtLocation` "/Game/Audio/SFX/Environment/Light/SC_LightFlicker_2.SC_LightFlicker_2" _returnvalue_2 (struct) 1.0 _returnvalue 0.0 null null null null)
        (bind (_direction _newtrack_0) (`Timeline|Timeline_0` :!label _label)
          (:`Update`
            (if (not (`self.Force Stop?`))
              (`self.Set All Intensity` (* (`KismetMathLibrary.MapRangeClamped` (`KismetMathLibrary.Sin` (* (`KismetMathLibrary.RandomFloatInRange` 0.5 3.0) _newtrack_0)) -1.0 1.0 4000.0 (`self.Default Intensity`)) (`KismetMathLibrary.RandomFloatInRange` 0.0 1.0)))))
          (:`Finished`
            (`self.Set All Intensity` (`self.Default Intensity`))
            (`KismetSystemLibrary.K2_SetTimerDelegate` (delegate `Flicker`) (`KismetMathLibrary.RandomFloatInRange` 1.0 5.0) :!label _label_2))))
      (:`B`
        (`GameplayStatics.PlaySoundAtLocation` "/Game/Audio/SFX/Environment/Light/SC_LightFlicker_1.SC_LightFlicker_1" _returnvalue_2 (struct) 1.0 _returnvalue 0.0 null null null null)
        (goto _label :!via `Reverse`)))))

(event `break`
  ;[1 1 1] Flicker
  (goto _label :!via `Stop`))

(event `Start Flicker Loop`
  ;[1 1 1] Flicker
  (goto _label_2))

(fn `Set All Intensity`
  (params (Intensity :type "Float (double-precision)"))
  (`LightComponent.SetIntensity` (`self.SpotLight`) Intensity)
  (message `AudioParameterControllerInterface.SetFloatParameter` (`self.material`) "emi" (`KismetMathLibrary.MapRangeClamped` Intensity 4000.0 (`self.Default Intensity`) 0.0 1.0)))

(fn `UserConstructionScript`
  (if (`self.on?`)
    (`self.Set All Intensity` (`self.Default Intensity`))))