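; Station actor ("stationEntiere") that animates itself with timeline-driven rotation from BeginPlay.
; One timeline turns the SMGasDynamicTrap1Part1 component around world roll, keeping its current pitch and yaw.
; A second, slower timeline rotates DefaultSceneRoot in both pitch and yaw from the same track, keeping its roll.
; Each track value is scaled to degrees of a full turn, and the construction script is empty.
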(event `self.ReceiveBeginPlay`
  (bind _sm_gasdynamictrap1_part1 (`self.SM_GasDynamicTrap1_part1`))
  (bind _defaultsceneroot (`self.DefaultSceneRoot`))
  (bind _returnvalue_roll (`KismetMathLibrary.BreakRotator` (`SceneComponent.K2_GetComponentRotation` _defaultsceneroot)))
  (bind (_returnvalue_roll_2 _returnvalue_pitch _returnvalue_yaw) (`KismetMathLibrary.BreakRotator` (`SceneComponent.K2_GetComponentRotation` _sm_gasdynamictrap1_part1)))
  (`|ExecutionSequence`
    (:`then_0`
      (`TimelineComponent.SetPlayRate` (`self.Timeline_0`) 0.4)
      (bind (_direction _newtrack_0) (`Timeline|Timeline_0`)
        (:`Update`
          (`SceneComponent.K2_SetWorldRotation` _sm_gasdynamictrap1_part1 (`KismetMathLibrary.MakeRotator` (* _newtrack_0 360.0) _returnvalue_pitch _returnvalue_yaw) false false))))
    (:`then_1`
      (`TimelineComponent.SetPlayRate` (`self.2`) 0.1)
      (bind (_direction_2 _newtrack_0_2) (`Timeline|2`)
        (:`Update`
          (bind _returnvalue (* _newtrack_0_2 360.0))
          (`SceneComponent.K2_SetWorldRotation` _defaultsceneroot (`KismetMathLibrary.MakeRotator` _returnvalue_roll _returnvalue _returnvalue) false false))))))

(fn `UserConstructionScript`)