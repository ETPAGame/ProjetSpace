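; Sound manager actor that switches background music and player breathing loops through volume changes.
; BeginPlay spawns three music tracks and normal and zero-G breath sounds as 2D audio, then mutes all five.
; MusicChanger crossfades between tracks, while ChangePlayerBreath instantly selects normal, zero-G or no breath, each comparing an integer state to 1.
; Both print debug labels, and their calls in the event graph are unconnected.
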(event `self.ReceiveBeginPlay`
  (`|ExecutionSequence`
    (:`then_0`
      (bind _returnvalue (`GameplayStatics.SpawnSound2D` "/Game/Pack/StarterContent/Audio/Starter_Music01.Starter_Music01" 1.0 1.0 0.0 null false false))
      (bind _output_get (set `self.Music_Ambiance_01` _returnvalue)))
    (:`then_1`
      (bind _returnvalue_2 (`GameplayStatics.SpawnSound2D` "/Game/Audio/Music/Music_Credit_v1.Music_Credit_v1" 1.0 1.0 0.0 null false false))
      (bind _output_get_2 (set `self.Music_Ambience_02` _returnvalue_2)))
    (:`then_2`
      (bind _returnvalue_3 (`GameplayStatics.SpawnSound2D` "/Game/Audio/Music/Music_Test.Music_Test" 1.0 1.0 0.0 null false false))
      (bind _output_get_3 (set `self.Music_Ambiance_03` _returnvalue_3)))
    (:`then_3`
      (bind _returnvalue_4 (`GameplayStatics.SpawnSound2D` "/Game/Audio/SFX/Player/Breath/Player_Breath_0G_Off.Player_Breath_0G_Off" 1.0 1.0 0.0 null false false))
      (bind _output_get_4 (set `self.Breath_Normal` _returnvalue_4)))
    (:`then_4`
      (bind _returnvalue_5 (`GameplayStatics.SpawnSound2D` "/Game/Audio/SFX/Player/Breath/Player_Breath_0G_On.Player_Breath_0G_On" 1.0 1.0 0.0 null false false))
      (bind _output_get_5 (set `self.Breath_0G` _returnvalue_5))
      (`AudioComponent.AdjustVolume` _output_get_5 0.0 0.0 "SCurve")
      (`AudioComponent.AdjustVolume` _output_get_4 0.0 0.0 "SCurve")
      (`AudioComponent.AdjustVolume` _output_get_3 0.0 0.0 "SCurve")
      (`AudioComponent.AdjustVolume` _output_get_2 0.0 0.0 "SCurve")
      (`AudioComponent.AdjustVolume` _output_get 0.0 0.0 "SCurve"))))

(fn `Change Player Breath`
  (params (BreathState :type Integer))
  (bind _breath_normal (`self.Breath_Normal`))
  (bind _breath_0g (`self.Breath_0G`))
  (`/Engine/EditorBlueprintResources/StandardMacros.DoOnce` false
    (:`Completed`
      (`/Engine/EditorBlueprintResources/StandardMacros.CompareInt` BreathState 1
        (:`>`
          (`AudioComponent.AdjustVolume` _breath_normal 0.0 0.0 "SCurve")
          (`AudioComponent.AdjustVolume` _breath_0g 0.0 0.0 "SCurve")
          (`KismetSystemLibrary.PrintString` "No breath"))
        (:`==`
          (`AudioComponent.AdjustVolume` _breath_normal 0.0 0.5 "SCurve")
          (`AudioComponent.AdjustVolume` _breath_0g 0.0 0.0 "SCurve")
          (`KismetSystemLibrary.PrintString` "Breath normal"))
        (:`<`
          (`AudioComponent.AdjustVolume` _breath_0g 0.0 0.5 "SCurve")
          (`AudioComponent.AdjustVolume` _breath_normal 0.0 0.0 "SCurve")
          (`KismetSystemLibrary.PrintString` "Breath 0G"))))))

(fn `MusicChanger`
  (params (MusicState :type Integer))
  (`/Engine/EditorBlueprintResources/StandardMacros.DoOnce` false
    (:`Completed`
      (`/Engine/EditorBlueprintResources/StandardMacros.CompareInt` MusicState 1
        (:`>`
          (`AudioComponent.AdjustVolume` (`self.Music_Ambiance_01`) 1.0 0.5 "SCurve")
          (`AudioComponent.AdjustVolume` (`self.Music_Ambience_02`) 0.5 0.0 "SCurve")
          (`AudioComponent.AdjustVolume` (`self.Music_Ambiance_03`) 0.5 0.0 "SCurve")
          (`KismetSystemLibrary.PrintString` "Music 1"))
        (:`==`
          (`AudioComponent.AdjustVolume` (`self.Music_Ambience_02`) 1.0 0.5 "SCurve")
          (`AudioComponent.AdjustVolume` (`self.Music_Ambiance_01`) 0.5 0.0 "SCurve")
          (`AudioComponent.AdjustVolume` (`self.Music_Ambiance_03`) 0.5 0.0 "SCurve")
          (`KismetSystemLibrary.PrintString` "Music 2"))
        (:`<`
          (`AudioComponent.AdjustVolume` (`self.Music_Ambiance_03`) 1.0 0.5 "SCurve")
          (`AudioComponent.AdjustVolume` (`self.Music_Ambiance_01`) 0.5 0.0 "SCurve")
          (`AudioComponent.AdjustVolume` (`self.Music_Ambience_02`) 0.5 0.0 "SCurve")
          (`KismetSystemLibrary.PrintString` "Music 3"))))))

(fn `UserConstructionScript`)