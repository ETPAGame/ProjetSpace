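; Flickering neon light actor with two rect lights, the second at half intensity, that starts dark when play begins.
; Switch alternates between starting the flicker and forcing both lights off.
; Flicker alternately plays and reverses a timeline that drives randomized sine-based intensity with a pitch-varied neon sound, restores default intensity when finished, then re-triggers itself on a random timer.
; StartFlickerLoop schedules that loop directly; the demo calls are disconnected.
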(event `self.ReceiveBeginPlay`
  (`LightComponent.SetIntensity` (`self.RectLight`) 0.0)
  (`LightComponent.SetIntensity` (`self.RectLight1`) 0.0))

(event `Switch`
  ;[1 1 1] Switch Mode
  (`/Engine/EditorBlueprintResources/StandardMacros.FlipFlop`
    (:`A`
      (set `self.ForceStop?` false)
      (`self.Flicker`))
    (:`B`
      (set `self.ForceStop?` true)
      (`self.Set All Intensity` 0.0)
      (`self.break`))))

(event `Flicker`
  (bind _returnvalue (`KismetMathLibrary.RandomFloatInRange` 0.9 1.1))
  (bind _returnvalue_2 (`SceneComponent.K2_GetComponentLocation` (`self.RectLight`)))
  ;[1 1 1] Flicker
  (if (not (`self.ForceStop?`))
    (`/Engine/EditorBlueprintResources/StandardMacros.FlipFlop`
      (:`A`
        (`KismetSystemLibrary.Delay` (`KismetMathLibrary.RandomFloatInRange` 0.0 2.0))
        (`GameplayStatics.PlaySoundAtLocation` "/Game/Audio/SFX/Environment/Light/Neon/SC_TurnOn_Neon_01.SC_TurnOn_Neon_01" _returnvalue_2 (struct) 0.5 _returnvalue 0.0 null null null null)
        (bind (_direction _newtrack_0) (`Timeline|Flick` :!label _label)
          (:`Update`
            (if (not (`self.ForceStop?`))
              (`self.Set All Intensity` (* (`KismetMathLibrary.MapRangeClamped` (`KismetMathLibrary.Sin` (* (`KismetMathLibrary.RandomFloatInRange` 0.5 3.0) _newtrack_0)) -1.0 1.0 4000.0 (`self.Default Intensity`)) (`KismetMathLibrary.RandomFloatInRange` 0.0 1.0)))))
          (:`Finished`
            (`self.Set All Intensity` (`self.Default Intensity`))
            (`KismetSystemLibrary.K2_SetTimerDelegate` (delegate `Flicker`) (`KismetMathLibrary.RandomFloatInRange` 1.0 5.0) :!label _label_2))))
      (:`B`
        (`GameplayStatics.PlaySoundAtLocation` "/Game/Audio/SFX/Environment/Light/Neon/SC_TurnOn_Neon_01.SC_TurnOn_Neon_01" _returnvalue_2 (struct) 0.5 _returnvalue 0.0 null null null null)
        (goto _label :!via `Reverse`)))))

(event `break`
  ;[1 1 1] Flicker
  (goto _label :!via `Stop`))

(event `Start Flicker Loop`
  ;[1 1 1] Flicker
  (goto _label_2))

(fn `Set All Intensity`
  (params (Intensity :type "Float (double-precision)"))
  (`LightComponent.SetIntensity` (`self.RectLight`) Intensity)
  (`LightComponent.SetIntensity` (`self.RectLight1`) (/ Intensity 2.0)))

(fn `UserConstructionScript`
  (if (`self.on?`)
    (`self.Set All Intensity` (`self.Default Intensity`))))