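; Evacuation manager actor that switches its wired neon meshes, rect lights and a separate light into a warning state.
; BeginPlay enables its World Partition streaming source.
; The WARNING event swaps a material slot on each neon mesh to red emissive, sets rect light intensity and shows the light.
; The construction script draws splines from each wired actor to the manager's root, visualizing the links.
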(event `self.ReceiveBeginPlay`
  (`WorldPartitionStreamingSourceComponent.EnableStreamingSource` (`self.WorldPartitionStreamingSource`)))

(event `WARNING`
  (for _array_element (`self.NeonWired`)
    (bind _asstatic_mesh_actor (cast `StaticMeshActor` _array_element))
    (`PrimitiveComponent.SetMaterial` (`StaticMeshActor.StaticMeshComponent` _asstatic_mesh_actor) 1 "/Game/Material/M_TEMP_RedEmissive1.M_TEMP_RedEmissive1"))
  (for _array_element_2 (`self.RectWired`)
    (`LightComponent.SetIntensity` (`RectLight.RectLightComponent` _array_element_2) 50.0))
  (`SceneComponent.SetVisibility` (`Light.LightComponent` (`self.Light`)) true true))

(fn `UserConstructionScript`
  ;[1 0.5141 0.9922] Draw Link
  (for _array_element (`self.NeonWired`)
    (`/Engine/EditorBlueprintResources/StandardMacros.IsValid` _array_element
      (:`Is Valid`
        (bind _returnvalue (`AddComponent|NODE_AddSplineComponent-0`))
        (`SplineComponent.SetSplinePoints` _returnvalue (`|MakeArray` (`self.K2_GetActorLocation` _array_element) (`SceneComponent.K2_GetComponentLocation` (`self.DefaultSceneRoot`))) "World" true))))
  (for _array_element_2 (`self.RectWired`)
    (`/Engine/EditorBlueprintResources/StandardMacros.IsValid` _array_element_2
      (:`Is Valid`
        (bind _returnvalue_2 (`AddComponent|NODE_AddSplineComponent-1`))
        (`SplineComponent.SetSplinePoints` _returnvalue_2 (`|MakeArray` (`self.K2_GetActorLocation` _array_element_2) (`SceneComponent.K2_GetComponentLocation` (`self.DefaultSceneRoot`))) "World" true)))))