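; Dialogue manager Blueprint that plays indexed voice lines from a dialogue table, with optional subtitles sent to the player character's HUD.
; PlayAudio plays one line at a time, holding for its delay before following its Next link or, if none, pulling the oldest queued ID.
; Requests arriving during playback join the queue without duplicates.
; A looping timer prints the queue as debug output.
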(event `GetRef`
  (bind _asbp_first_person_character (cast `/Game/Blueprint/BP_FirstPersonCharacter` (`GameplayStatics.GetPlayerCharacter` 0)))
  (set `self.HUDRef` (`/Game/Blueprint/BP_FirstPersonCharacter.HUDRef` _asbp_first_person_character)))

(event `PlayAudio`
  (params (IdSound :type Integer))
  (bind _id_sound (`self.Id Sound`))
  (bind _cue (`self.Cue`))
  (bind (_output_text _output_audio _output_delay _output_next) (break `/Game/Struct_Dialogue` (`|GetArrayItem` (`self.DialogueTab`) _id_sound)))
  (if (`self.IsAvailable`)
    (set `self.Id Sound` IdSound)
    (set `self.IsAvailable` false)
    (`|ExecutionSequence`
      (:`then_0`
        (if (`self.Subtitle?`)
          (`self.ShowSubtitle` _id_sound)))
      (:`then_1`
        (`GameplayStatics.PlaySound2D` _output_audio 1.0 1.0 0.0 null null))
      (:`then_2`
        (`KismetSystemLibrary.Delay` _output_delay)
        (set `self.IsAvailable` true)
        (if (!= _output_next 0)
          (`self.PlayAudio` _output_next)
          (elif (!= (`KismetArrayLibrary.Array_Length` (`self.Cue`)) 0)
            (bind _output_get (set `self.Temp` (`|GetArrayItem` _cue)))
            (`KismetArrayLibrary.Array_Remove` _cue)
            (`self.PlayAudio` _output_get)))))
    (else
      (`KismetArrayLibrary.Array_AddUnique` (`self.Cue`) IdSound))))

(event `ShowSubtitle`
  (params (IdSub :type Integer))
  (bind (_output_text _output_audio _output_delay) (break `/Game/Struct_Dialogue` (`|GetArrayItem` (`self.DialogueTab`) IdSub)))
  (`/Game/WPB_HUDInGame.ShowSubtitle` (`self.HUDRef`) _output_delay _output_text))

(event `self.ReceiveBeginPlay`
  (`KismetSystemLibrary.K2_SetTimerDelegate` (delegate `CustomEvent_0`) 2.0 true))

(event `CustomEvent_0`
  (for _array_element (`self.Cue`)
    (`KismetSystemLibrary.PrintString` (`KismetStringLibrary.Conv_IntToString` _array_element))))

(fn `UserConstructionScript`)