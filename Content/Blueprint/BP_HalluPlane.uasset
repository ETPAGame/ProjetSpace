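; BP_HalluPlane runs an escalating hallucination sequence that flashes a monster in front of the player.
; Hallu re-calls itself after per-step Timer delays; TPMONSTRE places the monster at indexed Distance along the player's forward vector, yaws it toward them and plays a violin sting.
; Each appearance briefly lingers before dropping below the actor.
; After four, a placeholder death-cinematic print precedes teleporting the player, setting fog density and calling the character's HalluLoop.
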(event `Hallu`
  (params (Duration :type "Float (single-precision)"))
  (bind _returnvalue (`GameplayStatics.GetPlayerCharacter` 0))
  (bind _returnvalue_2 (+ (`self.numberHallu`) 1))
  (if (>= (`self.numberHallu`) 4)
    (`KismetSystemLibrary.PrintString` "cinématique mort")
    (`KismetSystemLibrary.Delay` 2.0)
    (`self.K2_TeleportTo` :`self` _returnvalue :`DestLocation` (-9944.589844 40848.191406 -1305.936157))
    (bind _returnvalue_3 (`GameplayStatics.GetActorOfClass` "/Script/Engine.ExponentialHeightFog"))
    (`ExponentialHeightFogComponent.SetFogDensity` (`ExponentialHeightFog.Component` _returnvalue_3) 0.01)
    (bind _asbp_first_person_character (cast `/Game/Blueprint/BP_FirstPersonCharacter` _returnvalue))
    (`/Game/Blueprint/BP_FirstPersonCharacter.halluLoop` _asbp_first_person_character)
    (else
      (`KismetSystemLibrary.Delay` Duration)
      (`KismetSystemLibrary.PrintString` "tick")
      (`self.TP MONSTRE` _returnvalue_2)
      (`KismetSystemLibrary.Delay` 0.2)
      (`SceneComponent.K2_SetRelativeLocation` (`self.monstre`) (0.0 0.0 -500.0) false false)
      (bind _output_get (set `self.numberHallu` _returnvalue_2))
      (`self.Hallu` (`|GetArrayItem` (`self.timer`) _output_get)))))

(fn `TP MONSTRE`
  (params (index :type Integer))
  (bind _returnvalue (`GameplayStatics.GetPlayerCharacter` 0))
  (bind _monstre (`self.monstre`))
  (bind (_returnvalue_x _returnvalue_y _returnvalue_z) (`KismetMathLibrary.BreakVector` (`SceneComponent.K2_GetComponentLocation` (`self.DefaultSceneRoot`))))
  (bind _output (`|GetArrayItem` (`self.distance`) index))
  (bind _returnvalue_2 (`SceneComponent.K2_GetComponentLocation` (`Character.CapsuleComponent` _returnvalue)))
  (bind (_returnvalue_roll _returnvalue_pitch _returnvalue_yaw) (`KismetMathLibrary.BreakRotator` (`KismetMathLibrary.FindLookAtRotation` (`SceneComponent.K2_GetComponentLocation` _monstre) _returnvalue_2)))
  (bind (_returnvalue_x_2 _returnvalue_y_2) (`KismetMathLibrary.BreakVector` (+ (* (`SceneComponent.GetForwardVector` (`Character.CapsuleComponent` _returnvalue)) _output) _returnvalue_2)))
  (`KismetSystemLibrary.PrintString` (`KismetStringLibrary.Conv_DoubleToString` _output))
  (`SceneComponent.K2_SetWorldLocation` _monstre (`KismetMathLibrary.MakeVector` _returnvalue_x_2 _returnvalue_y_2 _returnvalue_z) false false)
  (`SceneComponent.K2_SetWorldRotation` (`self.monstre`) (`KismetMathLibrary.MakeRotator` 0.0 0.0 (- _returnvalue_yaw 90.0)) false false)
  (`GameplayStatics.PlaySound2D` "/Game/Audio/Ambiance/Sfx_Ambiance_Jumpscare_Violin.Sfx_Ambiance_Jumpscare_Violin" 1.0 (`KismetMathLibrary.RandomFloatInRange` 0.9 1.1) 0.0 null null))

(fn `UserConstructionScript`)