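; Grabbable power cable that the player plugs into a socket to activate wired actors, with support for zero-gravity play.
; Interaction hands the plug to the first-person or zero-G pawn, with physics and collision setup depending on the Gravity flag.
; Socket overlap snaps the plug, releases it, stops the timeline-driven light and sparks, lights the cable material and messages WiredItems through BPI_WiredActor.
; The construction script draws spline links to each wired item.
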(event `self.ReceiveBeginPlay`
  (bind _prisecable (`self.PriseCable`))
  (if (not (`self.gravity?`))
    (`PrimitiveComponent.SetSimulatePhysics` _prisecable true)
    (`PrimitiveComponent.SetEnableGravity` _prisecable false)
    (`PrimitiveComponent.SetCollisionResponseToChannel` _prisecable "ECC_Pawn" "ECR_Block"))
  (bind _returnvalue (`KismetMaterialLibrary.CreateDynamicMaterialInstance` "/Game/Material/M_Cable.M_Cable"))
  (bind _output_get (set `self.MI_cable` _returnvalue))
  (`PrimitiveComponent.SetMaterial` (`self.Cable1`) 0 _output_get)
  (bind (_direction _newtrack_0) (`Timeline|Timeline_0` :!label _label)
    (:`Update`
      (`LightComponent.SetIntensity` (`self.PointLight`) (* _newtrack_0 2000.0)))))

(event `break`
  (`|ExecutionSequence`
    (:`then_0`
      (goto _label :!via `Stop`))
    (:`then_1`
      (`LightComponent.SetIntensity` (`self.PointLight`) 0.0))))

(event `/Game/Inputs/BPI_Interact.Interaction`
  (params (itemToGrab :type "PrimitiveComponent Object Reference") (PlayerREF :type "Actor Object Reference"))
  (bind _prisecable (`self.PriseCable`))
  (bind _prisecable_2 (`self.PriseCable`))
  ;[1 1 1] interaction
  (if (`self.attached?`)
    _
    (elif (== itemToGrab (`self.PriseCable`))
      (if (not (`self.gravity?`))
        (`PrimitiveComponent.SetCollisionResponseToChannel` _prisecable "ECC_Pawn" "ECR_Overlap"))
      (bind _output_get (set `self.Player REF` PlayerREF))
      (`PrimitiveComponent.SetSimulatePhysics` _prisecable true)
      (bind _asbp_first_person_character (cast `/Game/Blueprint/BP_FirstPersonCharacter` _output_get)
        (:`then`
          (`/Game/Blueprint/BP_FirstPersonCharacter.GRABBING` _asbp_first_person_character _prisecable_2)
          (set `self.grab?` true)
          (set `ActorComponent.ComponentTags` (`|MakeArray` "None" :!type "Name") (`self.PriseCable`)))
        (:`CastFailed`
          (bind _asbp_zero_gpawn_cam (cast `/Game/Blueprint/BP_ZeroGPawnCam` _output_get))
          (`/Game/Blueprint/BP_ZeroGPawnCam.GRABBING` _asbp_zero_gpawn_cam _prisecable_2)
          (set `ActorComponent.ComponentTags` (`|MakeArray` "None" :!type "Name") (`self.PriseCable`)))))))

(event `deletePlug`
  ;[1 1 1] delete
  (if (not (`self.attached?`))
    (`ActorComponent.K2_DestroyComponent` (`self.Plug`))
    (`CableComponent.SetAttachEndToComponent` (`self.Cable1`) (`self.1`) "None")))

(event `attached`
  (params (Index :type Integer))
  (bind _prisecable (`self.PriseCable`))
  (bind _2 (`self.2`))
  (bind _player_ref (`self.Player REF`))
  (bind (_returnvalue_roll _returnvalue_pitch _returnvalue_yaw) (`KismetMathLibrary.BreakRotator` (`SceneComponent.K2_GetComponentRotation` _2)))
  ;[1 1 1] attached
  (`self.break`)
  (`NiagaraComponent.SetVariableFloat` (`self.NS_Sparkles1`) "spawnCount" 0.0)
  (`NiagaraComponent.SetVariableFloat` (`self.NS_Sparkles`) "spawnCount" 0.0)
  (`PrimitiveComponent.SetSimulatePhysics` _prisecable false)
  (`SceneComponent.K2_SetWorldLocation` _prisecable (`SceneComponent.K2_GetComponentLocation` _2) false false)
  (`SceneComponent.K2_SetWorldRotation` _prisecable (`KismetMathLibrary.MakeRotator` (+ _returnvalue_roll 90.0) _returnvalue_pitch _returnvalue_yaw) false false)
  (`MaterialInstanceDynamic.SetScalarParameterValue` (`self.MI_cable`) "on?" 1.0)
  (bind _asbp_first_person_character (cast `/Game/Blueprint/BP_FirstPersonCharacter` _player_ref)
    (:`then`
      (`/Game/Blueprint/BP_FirstPersonCharacter.Ungrab` _asbp_first_person_character null))
    (:`CastFailed`
      (bind _asbp_zero_gpawn_cam (cast `/Game/Blueprint/BP_ZeroGPawnCam` _player_ref))
      (`/Game/Blueprint/BP_ZeroGPawnCam.Ungrab` _asbp_zero_gpawn_cam null)))
  (for _array_element (`self.WiredItems`)
    (if (`KismetSystemLibrary.DoesImplementInterface` _array_element "/Game/Blueprint/BPI_WiredActor.BPI_WiredActor_C")
      (`GameplayStatics.PlaySoundAtLocation` "/Game/Audio/SFX/Environment/Interactible/SC_Button.SC_Button" (`SceneComponent.K2_GetComponentLocation` (`self.StaticMesh1`)) (struct) 0.5 1.0 0.0 null null null null)
      (message `/Game/Blueprint/BPI_WiredActor.WiredAction` _array_element))))

(event `self.2.OnComponentBeginOverlap`
  (params (OverlappedComponent :type "PrimitiveComponent Object Reference") (OtherActor :type "Actor Object Reference") (OtherComp :type "PrimitiveComponent Object Reference") (OtherBodyIndex :type Integer) (bFromSweep :type Boolean) (SweepResult :type "HitResult Structure (by ref)"))
  ;[1 1 1] overlap attach
  (if (== OtherComp (`self.PriseCable`))
    (`self.attached` 1)
    (set `self.attached?` true)
    (if (`self.StaticMesh To Switch?`)
      (for _array_element (`self.SM`)
        (`/Game/Blueprint/BP_WallToColor.Color` _array_element)))))

(event `self.PriseCable.OnComponentHit`
  (params (HitComponent :type "PrimitiveComponent Object Reference") (OtherActor :type "Actor Object Reference") (OtherComp :type "PrimitiveComponent Object Reference") (NormalImpulse :type "Vector Structure") (Hit :type "HitResult Structure (by ref)"))
  (cast `/Game/Blueprint/BP_ZeroGPawnCam` OtherActor)
  (`PrimitiveComponent.WakeRigidBody` (`self.PriseCable`) "None"))

(fn `UserConstructionScript`
  ;[1 0.5141 0.9922] Draw Link
  (for _array_element (`self.WiredItems`)
    (`/Engine/EditorBlueprintResources/StandardMacros.IsValid` _array_element
      (:`Is Valid`
        (bind _returnvalue (`AddComponent|NODE_AddSplineComponent-0`))
        (`SplineComponent.SetSplinePoints` _returnvalue (`|MakeArray` (`self.K2_GetActorLocation` _array_element) (`SceneComponent.K2_GetComponentLocation` (`self.1`))) "World" true)))))