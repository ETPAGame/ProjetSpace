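; Lab monster that travels along a per-room spline and kills the zero-G player pawn when it gets close.
; FollowSpline drives location and rotation through a Timeline at that spline's speed, while a looping timer checks player distance.
; A catch locks input, turns the player toward the monster's head, blends the view to it, plays a game-over animation, fades the HUD and retries the checkpoint.
; ResetActor offsets the monster far out of the level.
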(event `FollowSpline`
  (params (indexSalle :type Integer))
  (bind _output (`|GetArrayItem` (`self.SlineS`) indexSalle))
  (bind _spline (`/Game/Blueprint/BP_SplineMonsterLabs.Spline` _output))
  (bind _returnvalue (`KismetSystemLibrary.K2_SetTimerDelegate` (delegate `checkDistance`) 0.2 true))
  (`TimelineComponent.SetPlayRate` (`self.Timeline_0`) (`/Game/Blueprint/BP_SplineMonsterLabs.Speed` _output))
  (bind (_direction _newtrack_0) (`Timeline|Timeline_0` :!label _label)
    (:`Update`
      (`self.K2_SetActorLocation` self (`SplineComponent.GetLocationAtTime` _spline _newtrack_0 "World" false) false false)
      (bind (_returnvalue_roll _returnvalue_pitch _returnvalue_yaw) (`KismetMathLibrary.BreakRotator` (`SplineComponent.GetRotationAtTime` _spline _newtrack_0 "World" false)))
      (`self.K2_SetActorRotation` self (`KismetMathLibrary.MakeRotator` _returnvalue_roll _returnvalue_pitch _returnvalue_yaw) false))
    (:`Finished`
      (`self.stop`))))

(event `stop`
  (`KismetSystemLibrary.K2_PauseTimerHandle` (stale `FollowSpline` _returnvalue)))

(event `stopfollow`
  (goto _label :!via `Stop`))

(event `checkDistance`
  (bind _asbp_zero_gpawn_cam (cast `/Game/Blueprint/BP_ZeroGPawnCam` (`Controller.K2_GetPawn` (`GameplayStatics.GetPlayerController` 0))))
  (if (<= (`KismetMathLibrary.Vector_Distance` (`SceneComponent.K2_GetComponentLocation` (`/Game/Blueprint/BP_ZeroGPawnCam.Capsule` _asbp_zero_gpawn_cam)) (`SceneComponent.K2_GetComponentLocation` (`self.Scene`))) 900.0)
    (`self.dead`)))

(event `dead`
  (bind _returnvalue (`GameplayStatics.GetPlayerController` 0))
  (bind _returnvalue_2 (`KismetMathLibrary.FindLookAtRotation` (`self.K2_GetActorLocation` (`Controller.K2_GetPawn` _returnvalue)) (`SceneComponent.GetSocketLocation` (`self.SkeletalMesh`) "headSocket")))
  (`SkeletalMeshComponent.Stop` (`self.SkeletalMesh`))
  (bind _asbp_zero_gpawn_cam (cast `/Game/Blueprint/BP_ZeroGPawnCam` (`Controller.K2_GetPawn` (`GameplayStatics.GetPlayerController` 0))))
  (`SceneComponent.ResetRelativeTransform` (`self.SkeletalMesh`))
  (`self.DisableInput` _asbp_zero_gpawn_cam (`GameplayStatics.GetPlayerController` 0))
  (`self.K2_SetActorRotation` _asbp_zero_gpawn_cam _returnvalue_2 false)
  (`Controller.SetControlRotation` _returnvalue _returnvalue_2)
  (`SkeletalMeshComponent.PlayAnimation` (`self.SkeletalMesh`) "/Game/Monster/Animations/Gameover_Retargeted1.Gameover_Retargeted1" false)
  (`PlayerController.SetViewTargetWithBlend` (`GameplayStatics.GetPlayerController` 0) self 0.5 "VTBlend_Linear" 0.0 false)
  (`self.stopfollow`)
  (`self.stop`)
  (`KismetSystemLibrary.Delay` 1.1)
  (bind _asbp_player_controller (cast `/Game/Blueprint/BP_PlayerController` (`GameplayStatics.GetPlayerController` 0)))
  (`/Game/UserInterface/WPB_HUDInGame.fadeMort` (`/Game/Blueprint/BP_PlayerController.HUDRef` _asbp_player_controller))
  (`KismetSystemLibrary.Delay` 1.1)
  (bind _asbp_player_controller_2 (cast `/Game/Blueprint/BP_PlayerController` (`GameplayStatics.GetPlayerController` 0)))
  (`/Game/Blueprint/BP_PlayerController.Retry&Checkpoint` _asbp_player_controller_2 true)
  (`SkeletalMeshComponent.PlayAnimation` (`self.SkeletalMesh`) "/Game/Monster/Treading_Water__1__mixamo_com.Treading_Water__1__mixamo_com" true))

(event `/Game/Blueprint/BPI_WiredActor.ResetActor`
  (`SceneComponent.K2_AddWorldOffset` (`self.Scene`) (0.0 0.0 100000000.0) false false))

(fn `UserConstructionScript`)