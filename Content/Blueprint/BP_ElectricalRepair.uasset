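; BP_ElectricalRepair is an interactable electrical actor that triggers a set of linked actors a single time.
; On the first Interaction, it loops through WiredItems, setting RectLight intensity to zero and sending WiredActionMessage to other actors implementing BPI_WiredActor.
; The construction script adds a two-point spline from each valid wired item to the actor's root, visualizing the links.
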(event `/Game/Inputs/BPI_Interact.Interaction`
  (params (itemToGrab :type "PrimitiveComponent Object Reference") (PlayerREF :type "/Game/Blueprint/BP_FirstPersonCharacter Object Reference"))
  (`/Engine/EditorBlueprintResources/StandardMacros.DoOnce` false
    (:`Completed`
      (for _array_element (`self.WiredItems`)
        (bind _asrect_light (cast `RectLight` _array_element)
          (:`then`
            (`LightComponent.SetIntensity` (`Light.LightComponent` _asrect_light) 0.0))
          (:`CastFailed`
            (if (`KismetSystemLibrary.DoesImplementInterface` _array_element "/Game/Blueprint/BPI_WiredActor.BPI_WiredActor_C")
              (message `/Game/Blueprint/BPI_WiredActor.WiredAction` _array_element))))))))

(fn `UserConstructionScript`
  ;[1 0.5141 0.9922] Draw Link
  (for _array_element (`self.WiredItems`)
    (`/Engine/EditorBlueprintResources/StandardMacros.IsValid` _array_element
      (:`Is Valid`
        (bind _returnvalue (`AddComponent|NODE_AddSplineComponent-0`))
        (`SplineComponent.SetSplinePoints` _returnvalue (`|MakeArray` (`self.K2_GetActorLocation` _array_element) (`SceneComponent.K2_GetComponentLocation` (`self.DefaultSceneRoot`))) "World" true)))))