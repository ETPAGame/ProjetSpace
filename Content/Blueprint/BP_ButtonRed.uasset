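; Red button actor that, when interacted with, fires once to trigger every wired actor.
; A press nudges the button down, turns it green, plays sparkles and sound, then messages WiredItems implementing BPI_WiredActor.
; ResetActor restores the timeline-animated red emissive material, re-arms the DoOnce and propagates the reset to wired items.
; The construction script adds a spline to each valid wired item, visualizing the links.
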(event `/Game/Inputs/BPI_Interact.Interaction`
  (params (itemToGrab :type "PrimitiveComponent Object Reference") (PlayerREF :type "Actor Object Reference"))
  (bind _button (`self.Button`))
  (bind (_relativelocation_x _relativelocation_y _relativelocation_z) (`KismetMathLibrary.BreakVector` (`SceneComponent.RelativeLocation` _button)))
  (`/Engine/EditorBlueprintResources/StandardMacros.DoOnce` false :!label _label
    (:`Completed`
      (`SceneComponent.K2_SetRelativeLocation` _button (`KismetMathLibrary.MakeVector` _relativelocation_x (- _relativelocation_y 1.0) _relativelocation_z) false false)
      (`PrimitiveComponent.SetMaterial` (`self.Button`) 0 "/Game/Material/M_TEMP_GreenEmissive.M_TEMP_GreenEmissive")
      (`NiagaraComponent.ResetSystem` (`self.NS_Sparkles`))
      (`GameplayStatics.PlaySoundAtLocation` "/Game/Audio/SFX/Environment/Interactible/SC_Button.SC_Button" (`SceneComponent.K2_GetComponentLocation` (`self.Button`)) (struct) 0.6 1.0 0.0 null null null null)
      (for _array_element (`self.WiredItems`)
        (if (`KismetSystemLibrary.DoesImplementInterface` _array_element "/Game/Blueprint/BPI_WiredActor.BPI_WiredActor_C")
          (message `/Game/Blueprint/BPI_WiredActor.WiredAction` _array_element))))))

(event `Reset`
  (goto _label :!via `Reset`))

(event `self.ReceiveBeginPlay`
  (bind _returnvalue (`KismetMaterialLibrary.CreateDynamicMaterialInstance` "/Game/Material/M_TEMP_RedEmissive.M_TEMP_RedEmissive"))
  (bind _output_get (set `self.red emi` _returnvalue))
  (`PrimitiveComponent.SetMaterial` (`self.Button`) 0 _output_get)
  (`TimelineComponent.SetPlayRate` (`self.Timeline_0`) 0.5)
  (bind (_direction _newtrack_0) (`Timeline|Timeline_0` :!label _label_2)
    (:`Update`
      (`MaterialInstanceDynamic.SetScalarParameterValue` (`self.red emi`) "lerp" _newtrack_0))))

(event `/Game/Blueprint/BPI_WiredActor.ResetActor`
  (`PrimitiveComponent.SetMaterial` (`self.Button`) 0 (stale `self.ReceiveBeginPlay` _output_get))
  (`self.Reset`)
  (for _array_element (`self.WiredItems`)
    (message `/Game/Blueprint/BPI_WiredActor.ResetActor` _array_element))
  (goto _label_2))

(fn `UserConstructionScript`
  ;[1 0.5141 0.9922] Draw Link
  (`PrimitiveComponent.SetMaterial` (`self.Button`) 0 "/Game/Material/M_TEMP_RedEmissive.M_TEMP_RedEmissive")
  (for _array_element (`self.WiredItems`)
    (`/Engine/EditorBlueprintResources/StandardMacros.IsValid` _array_element
      (:`Is Valid`
        (bind _returnvalue (`AddComponent|NODE_AddSplineComponent-0`))
        (`SplineComponent.SetSplinePoints` _returnvalue (`|MakeArray` (`self.K2_GetActorLocation` _array_element) (`SceneComponent.K2_GetComponentLocation` (`self.DefaultSceneRoot`))) "World" true)))))