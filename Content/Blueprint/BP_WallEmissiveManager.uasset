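; BP_WallEmissiveManager is a manager actor that switches off the emissive look and lighting of a group of wired walls.
; Its Eteindre event applies a dark plastic material to two slots on each wall mesh, zeroes the linked spotlights, then calls SwitchLight on TurnOf with TurnOff set.
; The construction script draws a spline from each valid wall to the manager to show the links.
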(event `Eteindre`
  (bind _turnof (`self.TurnOf`))
  (for _array_element (`self.WiredWall`)
    (bind _asstatic_mesh_actor (cast `StaticMeshActor` _array_element))
    (bind _staticmeshcomponent (`StaticMeshActor.StaticMeshComponent` _asstatic_mesh_actor))
    (`PrimitiveComponent.SetMaterial` _staticmeshcomponent 4 "/Game/Material/MI_Plastic_Dark.MI_Plastic_Dark")
    (`PrimitiveComponent.SetMaterial` _staticmeshcomponent 1 "/Game/Material/MI_Plastic_Dark.MI_Plastic_Dark"))
  (for _array_element_2 (`self.Spotlight`)
    (`LightComponent.SetIntensity` (`SpotLight.SpotLightComponent` _array_element_2) 0.0))
  (set `/Game/Blueprint/BP_OnOffLight.turnOff` true _turnof)
  (`/Game/Blueprint/BP_OnOffLight.Switch Light` _turnof))

(fn `UserConstructionScript`
  ;[1 0.5141 0.9922] Draw Link
  (for _array_element (`self.WiredWall`)
    (`/Engine/EditorBlueprintResources/StandardMacros.IsValid` _array_element
      (:`Is Valid`
        (bind _returnvalue (`AddComponent|NODE_AddSplineComponent-0`))
        (`SplineComponent.SetSplinePoints` _returnvalue (`|MakeArray` (`self.K2_GetActorLocation` _array_element) (`SceneComponent.K2_GetComponentLocation` (`self.DefaultSceneRoot`))) "World" true)))))