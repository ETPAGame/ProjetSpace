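; Automatic three-panel lab door that opens for the first-person character or zero-G camera pawn when Openable is set.
; Box overlap begin and end both call Ouverture, which plays a pitch-randomized sound and flip-flops a SpeedDoor-rate timeline.
; The timeline slides Top, Left and Right panels from positions cached at BeginPlay.
; SwitchDecal, not called here, applies door-number glyph textures to either set of four decals through dynamic materials.
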(event `Ouverture`
  (bind (_leftloc_x _leftloc_y _leftloc_z) (`KismetMathLibrary.BreakVector` (`self.LeftLoc`)))
  (bind (_rightloc_x _rightloc_y _rightloc_z) (`KismetMathLibrary.BreakVector` (`self.RightLoc`)))
  (bind (_toploc_x _toploc_y _toploc_z) (`KismetMathLibrary.BreakVector` (`self.TopLoc`)))
  (`GameplayStatics.SpawnSoundAtLocation` null (`self.K2_GetActorLocation`) (struct) 1.0 (`KismetMathLibrary.RandomFloatInRange` 1.0 1.2) 0.0 null null false)
  (`TimelineComponent.SetPlayRate` (`self.Timeline_0`) (`self.SpeedDoor`))
  (`/Engine/EditorBlueprintResources/StandardMacros.FlipFlop`
    (:`A`
      (bind (_direction _newtrack_0) (`Timeline|Timeline_0` :!label _label)
        (:`Update`
          (`SceneComponent.K2_SetRelativeLocation` (`self.Top`) (`KismetMathLibrary.MakeVector` _toploc_x _toploc_y (+ _toploc_z (* (.x _newtrack_0) 100.0))) false false)
          (`SceneComponent.K2_SetRelativeLocation` (`self.Left`) (`KismetMathLibrary.MakeVector` (+ (* (.y _newtrack_0) -85.0) _leftloc_x) _leftloc_y _leftloc_z) false false)
          (`SceneComponent.K2_SetRelativeLocation` (`self.Right`) (`KismetMathLibrary.MakeVector` (+ (* (.z _newtrack_0) 85.0) _rightloc_x) _rightloc_y _rightloc_z) false false))))
    (:`B`
      (goto _label :!via `Reverse`))))

(event `self.ReceiveBeginPlay`
  (set `self.RightLoc` (`SceneComponent.RelativeLocation` (`self.Right`)))
  (set `self.LeftLoc` (`SceneComponent.RelativeLocation` (`self.Left`)))
  (set `self.TopLoc` (`SceneComponent.RelativeLocation` (`self.Top`))))

(event `self.Box.OnComponentBeginOverlap`
  (params (OverlappedComponent :type "PrimitiveComponent Object Reference") (OtherActor :type "Actor Object Reference") (OtherComp :type "PrimitiveComponent Object Reference") (OtherBodyIndex :type Integer) (bFromSweep :type Boolean) (SweepResult :type "HitResult Structure (by ref)"))
  (cast `/Game/Blueprint/BP_FirstPersonCharacter` OtherActor
    (:`then`
      _)
    (:`CastFailed`
      (cast `/Game/Blueprint/BP_ZeroGPawnCam` OtherActor)))
  (if (`self.Openable?`) :!label _label_2
    (`self.Ouverture`)))

(event `self.Box.OnComponentEndOverlap`
  (params (OverlappedComponent :type "PrimitiveComponent Object Reference") (OtherActor :type "Actor Object Reference") (OtherComp :type "PrimitiveComponent Object Reference") (OtherBodyIndex :type Integer))
  (cast `/Game/Blueprint/BP_FirstPersonCharacter` OtherActor
    (:`then`
      (goto _label_2))
    (:`CastFailed`
      (cast `/Game/Blueprint/BP_ZeroGPawnCam` OtherActor)
      (goto _label_2))))

(fn `SwitchDecal`
  (params (`01?` :type Boolean))
  (locals (`1?` :type Boolean))
  (bind _returnvalue (select `bool` (`local.1?`) :`false` (`self.MatDecal02`) :`true` (`self.MatDecal01`)))
  (set `local.1?` `01?`)
  (bind _returnvalue_2 (`KismetMaterialLibrary.CreateDynamicMaterialInstance` "/Game/UserInterface/GlypheSalle/DecalGlyphe_Inst.DecalGlyphe_Inst" "None"))
  (if (`local.1?`)
    (set `self.MatDecal01` _returnvalue_2)
    (else
      (set `self.MatDecal02` _returnvalue_2)))
  (`MaterialInstanceDynamic.SetTextureParameterValue` _returnvalue "Param" (select `int` (`KismetMathLibrary.SelectInt` (`self.NumeroPorte01`) (`self.NumeroPorte02`) (`local.1?`)) :`0` "/Game/UserInterface/GlypheSalle/1.1" :`1` "/Game/UserInterface/GlypheSalle/2.2" :`2` "/Game/UserInterface/GlypheSalle/3.3" :`3` "/Game/UserInterface/GlypheSalle/4.4" :`4` "/Game/UserInterface/GlypheSalle/5.5" :`5` "/Game/UserInterface/GlypheSalle/6.6" :`6` "/Game/UserInterface/GlypheSalle/7.7" :`7` "/Game/UserInterface/GlypheSalle/8.8" :`8` "/Game/UserInterface/GlypheSalle/9.9" :`9` "/Game/UserInterface/GlypheSalle/10.10" :`10` "/Game/UserInterface/GlypheSalle/11.11" :`11` "/Game/UserInterface/GlypheSalle/12.12" :`12` "/Game/UserInterface/GlypheSalle/13.13" :`13` "/Game/UserInterface/GlypheSalle/14.14" :`14` "/Game/UserInterface/GlypheSalle/15.15" :`15` "/Game/UserInterface/GlypheSalle/16.16" :`16` "/Game/UserInterface/GlypheSalle/17.17" :`17` "/Game/UserInterface/GlypheSalle/18.18" :!type "Texture Object Reference"))
  (`DecalComponent.SetDecalMaterial` (select `bool` (`local.1?`) :`false` (`self.Decal4`) :`true` (`self.Decal`)) _returnvalue)
  (`DecalComponent.SetDecalMaterial` (select `bool` (`local.1?`) :`false` (`self.Decal5`) :`true` (`self.Decal1`)) _returnvalue)
  (`DecalComponent.SetDecalMaterial` (select `bool` (`local.1?`) :`false` (`self.Decal6`) :`true` (`self.Decal2`)) _returnvalue)
  (`DecalComponent.SetDecalMaterial` (select `bool` (`local.1?`) :`false` (`self.Decal7`) :`true` (`self.Decal3`)) _returnvalue))

(fn `UserConstructionScript`)