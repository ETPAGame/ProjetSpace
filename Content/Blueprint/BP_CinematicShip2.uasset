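; BP_CinematicShip2 is a cinematic ship actor that handles sound and animated Niagara effects.
; BeginPlay starts its Audio component and plays two 2D sounds, including the cinematic start music.
; Custom on and off events run a timeline forward and in reverse, scaling its track into the "playrate" variable of both Niagara systems to ramp the effects up and down.
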(event `self.ReceiveBeginPlay`
  (`AudioComponent.Play` (`self.Audio`) 0.0)
  (`GameplayStatics.PlaySound2D` "/Game/Audio/Ambiance/59__fectoper__nostromo.59__fectoper__nostromo" 1.0 1.0 0.0 null null)
  (`GameplayStatics.PlaySound2D` "/Game/Audio/Music/Music_CinematicStart.Music_CinematicStart" 0.5 1.0 0.0 null null))

(event `on`
  (bind (_direction _newtrack_0) (`Timeline|Timeline_0` :!via `PlayFromStart` :!label _label)
    (:`Update`
      (`NiagaraComponent.SetVariableFloat` (`self.NewNiagaraEmitter_System`) "playrate" (* _newtrack_0 300.0))
      (`NiagaraComponent.SetVariableFloat` (`self.NewNiagaraEmitter_System1`) "playrate" (* _newtrack_0 300.0)))))

(event `off`
  (goto _label :!via `ReverseFromEnd`))

(fn `UserConstructionScript`)