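; Trigger-box actor that starts the player's breathing audio on overlap.
; The first overlap passes a DoOnce, then must be the first-person character or zero-G camera pawn to spawn fast and slow breath 2D sounds.
; A FlipFlop is meant to alternate them, but the DoOnce is never reset, so only the branch stopping slow and activating fast breathing runs.
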(event `self.Box.OnComponentBeginOverlap`
  (params (OverlappedComponent :type "PrimitiveComponent Object Reference") (OtherActor :type "Actor Object Reference") (OtherComp :type "PrimitiveComponent Object Reference") (OtherBodyIndex :type Integer) (bFromSweep :type Boolean) (SweepResult :type "HitResult Structure (by ref)"))
  (`/Engine/EditorBlueprintResources/StandardMacros.DoOnce` false
    (:`Completed`
      (cast `/Game/Blueprint/BP_FirstPersonCharacter` OtherActor
        (:`then`
          _)
        (:`CastFailed`
          (cast `/Game/Blueprint/BP_ZeroGPawnCam` OtherActor)))
      (bind _returnvalue (`GameplayStatics.SpawnSound2D` (`self.Breath_fast`) 1.0 1.0 0.0 null false false))
      (bind _returnvalue_2 (`GameplayStatics.SpawnSound2D` (`self.Breath_slow`) 1.0 1.0 0.0 null false false))
      (`/Engine/EditorBlueprintResources/StandardMacros.FlipFlop`
        (:`A`
          (`AudioComponent.Stop` _returnvalue_2)
          (`ActorComponent.SetActive` _returnvalue true false))
        (:`B`
          (`AudioComponent.Stop` _returnvalue)
          (`ActorComponent.SetActive` _returnvalue_2 true false))))))

(fn `UserConstructionScript`)