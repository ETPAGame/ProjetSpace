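; Trigger volume that advances the player's helmet damage and low-oxygen HUD feedback when a Pawn overlaps its box.
; Cassure selects one of three crack stages, calling the matching helmet-break and oxygen functions on BP_PlayerController's HUDRef, with the last stage also calling OxygeneLow.
; Each stage plays its own glass-cracking 2D sound.
; The graph never changes Cassure or disables the trigger, so every overlap replays the same stage.
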(event `self.Box.OnComponentBeginOverlap`
  (params (OverlappedComponent :type "PrimitiveComponent Object Reference") (OtherActor :type "Actor Object Reference") (OtherComp :type "PrimitiveComponent Object Reference") (OtherBodyIndex :type Integer) (bFromSweep :type Boolean) (SweepResult :type "HitResult Structure (by ref)"))
  (bind _cassure (`self.Cassure`))
  (cast `Pawn` OtherActor)
  (bind _asbp_player_controller (cast `/Game/Blueprint/BP_PlayerController` (`GameplayStatics.GetPlayerController` 0)))
  (switch `int` _cassure
    (:`0`
      (bind _hudref (`/Game/Blueprint/BP_PlayerController.HUDRef` _asbp_player_controller))
      (`/Game/UserInterface/WPB_HUDInGame.BreakHelmet` _hudref)
      (`/Game/UserInterface/WPB_HUDInGame.OxygenLowFollow` _hudref 0))
    (:`1`
      (`/Game/UserInterface/WPB_HUDInGame.BreakHelmetFollow` _hudref 0)
      (`/Game/UserInterface/WPB_HUDInGame.OxygenLowFollow` _hudref 1))
    (:`2`
      (`/Game/UserInterface/WPB_HUDInGame.BreakHelmetFollow` _hudref 1)
      (`/Game/UserInterface/WPB_HUDInGame.OxygenLowFollow` _hudref 2)
      (`/Game/UserInterface/WPB_HUDInGame.OxygeneLow` _hudref)))
  (`GameplayStatics.PlaySound2D` (select `int` _cassure :`0` "/Game/Audio/SFX/Player/Casque/CrackingGlass_01.CrackingGlass_01" :`1` "/Game/Audio/SFX/Player/Casque/Long_CrackingGlass_02.Long_CrackingGlass_02" :`2` "/Game/Audio/SFX/Player/Casque/Short_CrackingGlass_02.Short_CrackingGlass_02" :!type "SoundBase Object Reference") 0.7 1.0 0.0 null null))

(fn `UserConstructionScript`)