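; Trigger-volume actor that switches a wired set of flickering lights on and off as actors enter and leave its box.
; Begin overlap starts the flicker loop on each BP_FlickeringLight_2 in WiredLight and clears its ForceStop flag; end overlap sets that flag.
; Neither event filters the overlapping actor.
; The construction script draws a spline from each valid wired light to the manager's root, visualizing the links.
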(event `self.Box.OnComponentBeginOverlap`
  (params (OverlappedComponent :type "PrimitiveComponent Object Reference") (OtherActor :type "Actor Object Reference") (OtherComp :type "PrimitiveComponent Object Reference") (OtherBodyIndex :type Integer) (bFromSweep :type Boolean) (SweepResult :type "HitResult Structure (by ref)"))
  (for _array_element (`self.WiredLight`)
    (bind _asbp_flickering_light_2 (cast `/Game/Blueprint/BP_FlickeringLight_2` _array_element))
    (`/Game/Blueprint/BP_FlickeringLight_2.Start Flicker Loop` _asbp_flickering_light_2)
    (set `/Game/Blueprint/BP_FlickeringLight_2.ForceStop?` false _asbp_flickering_light_2)))

(event `self.Box.OnComponentEndOverlap`
  (params (OverlappedComponent :type "PrimitiveComponent Object Reference") (OtherActor :type "Actor Object Reference") (OtherComp :type "PrimitiveComponent Object Reference") (OtherBodyIndex :type Integer))
  (for _array_element (`self.WiredLight`)
    (bind _asbp_flickering_light_2 (cast `/Game/Blueprint/BP_FlickeringLight_2` _array_element))
    (set `/Game/Blueprint/BP_FlickeringLight_2.ForceStop?` true _asbp_flickering_light_2)))

(fn `UserConstructionScript`
  ;[1 0.5141 0.9922] Draw Link
  (for _array_element (`self.WiredLight`)
    (`/Engine/EditorBlueprintResources/StandardMacros.IsValid` _array_element
      (:`Is Valid`
        (bind _returnvalue (`AddComponent|NODE_AddSplineComponent-0`))
        (`SplineComponent.SetSplinePoints` _returnvalue (`|MakeArray` (`self.K2_GetActorLocation` _array_element) (`SceneComponent.K2_GetComponentLocation` (`self.DefaultSceneRoot`))) "World" true)))))