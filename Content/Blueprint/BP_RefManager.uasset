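; BP_RefManager is a Blueprint that hands the player's pawn to monster AI through their blackboards.
; When WiredAction fires, it waits briefly, then writes player zero's controlled pawn into the PlayerRef key of MonsterRef.
; It does the same for MonsterRef2, but only if both references are valid.
; A few debug prints remain in the graph, unconnected.
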(event `/Game/Blueprint/BPI_WiredActor.WiredAction`
  (bind _returnvalue (`KismetStringLibrary.Conv_StringToName` "PlayerRef"))
  (bind _monsterref (`self.MonsterRef`))
  (bind _monsterref2 (`self.MonsterRef2`))
  (bind _returnvalue_2 (`Controller.K2_GetPawn` (`GameplayStatics.GetPlayerController` 0)))
  (`KismetSystemLibrary.Delay` 1.5)
  (`/Engine/EditorBlueprintResources/StandardMacros.IsValid` _monsterref
    (:`Is Valid`
      (`BlackboardComponent.SetValueAsObject` (`AIBlueprintHelperLibrary.GetBlackboard` _monsterref) _returnvalue _returnvalue_2)
      (`/Engine/EditorBlueprintResources/StandardMacros.IsValid` _monsterref2
        (:`Is Valid`
          (`BlackboardComponent.SetValueAsObject` (`AIBlueprintHelperLibrary.GetBlackboard` _monsterref2) _returnvalue _returnvalue_2))))))

(fn `UserConstructionScript`)