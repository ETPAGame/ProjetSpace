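; GPS pointer actor that shows the player the direction and rough distance to an objective, hidden until activated.
; Activation caches the controlled pawn, reveals the actor and plays a timeline that rolls its inner scene component.
; Tick aims the actor along the pawn-to-objective vector and sets a chevron dynamic material parameter by three distance bands, with debug prints.
; NewObj copies the target from the zero-G pawn's Out value.
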(event `Activ`
  (bind (_relativerotation_roll _relativerotation_pitch _relativerotation_yaw) (`KismetMathLibrary.BreakRotator` (`SceneComponent.RelativeRotation` (`self.Scene`))))
  (`SceneComponent.SetVisibility` (`self.DefaultSceneRoot`) true true)
  (set `self.As BP First Person Character` (`Controller.K2_GetPawn` (`GameplayStatics.GetPlayerController` 0)))
  (bind (_direction _newtrack_0) (`Timeline|Timeline_0`)
    (:`Update`
      (`SceneComponent.K2_SetRelativeRotation` (`self.Scene`) (`KismetMathLibrary.MakeRotator` (* _newtrack_0 360.0) _relativerotation_pitch _relativerotation_yaw) false false))))

(event `Desactov`
  (`SceneComponent.SetVisibility` (`self.DefaultSceneRoot`) false true))

(event `self.ReceiveBeginPlay`
  (`self.Desactov`))

(event `CalcDist`
  (bind _returnvalue (`KismetMathLibrary.Vector_Distance` (`self.K2_GetActorLocation` (`self.As BP First Person Character`)) (`self.Objectif`)))
  (`KismetSystemLibrary.PrintString` (`KismetStringLibrary.Conv_DoubleToString` _returnvalue) true true (struct :`G` 0.66 :`B` 1.0 :`A` 1.0) 0.0)
  (if (> _returnvalue 1000.0)
    (set `self.Value` 0.672)
    (elif (< _returnvalue 500.0)
      (set `self.Value` 0.0)
      (else
        (set `self.Value` 0.16))))
  (`MaterialInstanceDynamic.SetScalarParameterValue` (`self.NewVar_0`) "Param" (`self.Value`)))

(event `self.ReceiveTick`
  (params (DeltaSeconds :type "Float (single-precision)"))
  (bind _returnvalue (`KismetMathLibrary.FindLookAtRotation` (`self.K2_GetActorLocation` (`self.As BP First Person Character`)) (`self.Objectif`)))
  (`/Engine/EditorBlueprintResources/StandardMacros.IsValid` (`self.As BP First Person Character`)
    (:`Is Valid`
      (`KismetSystemLibrary.PrintString` (`KismetStringLibrary.Conv_RotatorToString` _returnvalue) true true (struct :`R` 0.25 :`G` 0.146352 :`A` 1.0) 0.0)
      (`self.K2_SetActorRotation` _returnvalue)
      (`self.CalcDist`))))

(event `NewObj`
  (bind _asbp_zero_gpawn_cam (cast `/Game/Blueprint/BP_ZeroGPawnCam` (`self.As BP First Person Character`)))
  (set `self.Objectif` (`/Game/Blueprint/BP_ZeroGPawnCam.Out` _asbp_zero_gpawn_cam)))

(fn `UserConstructionScript`
  (bind _returnvalue (`PrimitiveComponent.CreateDynamicMaterialInstance` (`self.Chevrons`) 0 "/Game/ChevronsMat.ChevronsMat" "None"))
  (set `self.NewVar_0` _returnvalue))