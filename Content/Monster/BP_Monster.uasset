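; Monster that follows placed target points or tracks the player, then grabs and kills them on contact.
; UpdateDestination feeds each point's wait, teleport or tracking setting into AI Blackboard keys, while WiredAction interrupts or toggles movement.
; A sphere overlap fires a once-only kill that attaches the player to a mesh socket before death.
; The construction script previews the route as a spline, and ResetActor restores saved starting state.
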(event `self.ReceiveBeginPlay`
  (set `self.Action WTBReset` (`self.Action_WTB`))
  (set `self.Action KillReset` (`self.Action_Kill`))
  (set `self.Player RefReset` (`self.PlayerRef`))
  (set `self.Target ListReset` (`self.TargetList`))
  (set `self.Target Point MapReset` (`self.TargetPointMap`))
  (set `self.CurrentPoint` (`self.Current PointReset`))
  (set `self.Is MovingReset` (`self.IsMoving`))
  (set `self.Enable Move at StartReset` (`self.EnableMoveAtStart`))
  (set `self.Transofrm` (`self.GetTransform`))
  ;[1 1 1] Debug
  (if (`self.EnableMoveAtStart`)
    (`self.Update Destination`)))

(event `Update Destination`
  (bind _returnvalue (`AIBlueprintHelperLibrary.GetBlackboard` null))
  (bind _returnvalue_2 (`AIBlueprintHelperLibrary.GetBlackboard` null))
  (bind _returnvalue_3 (`KismetStringLibrary.Conv_StringToName` "IsFollowingPath"))
  (bind _currentpoint (`self.CurrentPoint`))
  (bind _targetlist (`self.TargetList`))
  (bind _output (`|GetArrayItem` _targetlist _currentpoint))
  (bind _returnvalue_4 (`self.K2_GetActorLocation` _output))
  (`/Engine/EditorBlueprintResources/StandardMacros.IsValid` _output
    (:`Is Valid`
      (if (`/Game/Blueprint/PATHPOINT.TrackingPlayer?` _output)
        (`BlackboardComponent.SetValueAsBool` _returnvalue_2 (`KismetStringLibrary.Conv_StringToName` "isTrackingPlayer") true)
        (`BlackboardComponent.SetValueAsBool` _returnvalue_2 _returnvalue_3 false)
        (else
          (set `self.IsMoving` false)
          (`BlackboardComponent.SetValueAsBool` _returnvalue_2 _returnvalue_3 false)
          (`KismetSystemLibrary.Delay` (`/Game/Blueprint/PATHPOINT.WaitTime` _output))
          (set `self.IsMoving` true)
          (`BlackboardComponent.SetValueAsBool` _returnvalue_2 _returnvalue_3 true)
          (if (< _currentpoint (`KismetArrayLibrary.Array_Length` _targetlist))
            (set `self.IsMoving` true)
            (if (`/Game/Blueprint/PATHPOINT.IsTeleport?` _output)
              (`self.K2_SetActorLocation` _returnvalue_4))
            (`BlackboardComponent.SetValueAsVector` _returnvalue (`KismetStringLibrary.Conv_StringToName` "CurrentTarget") _returnvalue_4)
            (`BlackboardComponent.SetValueAsBool` _returnvalue (`KismetStringLibrary.Conv_StringToName` "IsFollowingPath") true)
            (else
              (set `self.IsMoving` false))))))))

(event `Reset`
  (bind _returnvalue (`GameplayStatics.GetPlayerController` 0))
  (goto _label :!via `Reset`))

(event `self.Sphere.OnComponentBeginOverlap`
  (params (OverlappedComponent :type "PrimitiveComponent Object Reference") (OtherActor :type "Actor Object Reference") (OtherComp :type "PrimitiveComponent Object Reference") (OtherBodyIndex :type Integer) (bFromSweep :type Boolean) (SweepResult :type "HitResult Structure (by ref)"))
  (bind _returnvalue (`GameplayStatics.GetPlayerController` 0))
  (bind _asbp_first_person_character (cast `/Game/Blueprint/BP_FirstPersonCharacter` OtherActor)
    (:`then`
      _)
    (:`CastFailed`
      (cast `/Game/Blueprint/BP_ZeroGPawnCam` OtherActor)))
  (`/Engine/EditorBlueprintResources/StandardMacros.DoOnce` false :!label _label
    (:`Completed`
      (`KismetSystemLibrary.PrintString` "Kill")
      (`PrimitiveComponent.SetCollisionEnabled` (`Character.CapsuleComponent` _asbp_first_person_character) "NoCollision")
      (`BlackboardComponent.SetValueAsBool` (`AIBlueprintHelperLibrary.GetBlackboard` null) (`KismetStringLibrary.Conv_StringToName` "IsFollowingPath") false)
      (set `self.Action_Kill` true)
      (set `self.IsMoving` false)
      (set `self.PlayerRef` _asbp_first_person_character)
      (`self.DisableInput` _asbp_first_person_character _returnvalue)
      (`Controller.SetControlRotation` _returnvalue (`KismetMathLibrary.FindLookAtRotation` (`self.K2_GetActorLocation` (`Controller.K2_GetPawn` _returnvalue)) (`SceneComponent.GetSocketLocation` (`self.Mesh`) "GrabbedViewPoint")))
      (`self.K2_AttachToComponent` (`self.PlayerRef`) (`self.Mesh`) "GrabPoint" "SnapToTarget" "KeepRelative" "KeepRelative" true)
      (`KismetSystemLibrary.Delay` 2.2)
      (`/Game/Blueprint/BP_FirstPersonCharacter.PlayerDeath` _asbp_first_person_character))))

(event `/Game/Blueprint/BPI_WiredActor.WiredAction`
  (bind _returnvalue (`KismetStringLibrary.Conv_StringToName` "isTrackingPlayer"))
  (bind _returnvalue_2 (`AIBlueprintHelperLibrary.GetBlackboard` null))
  ;[1 1 1] Event Only : Skip to next target, resume movement by calling this again
  (if (`BlackboardComponent.GetValueAsBool` _returnvalue_2 _returnvalue)
    (`BlackboardComponent.SetValueAsBool` _returnvalue_2 _returnvalue false)
    (`BlackboardComponent.SetValueAsBool` _returnvalue_2 (`KismetStringLibrary.Conv_StringToName` "IsFollowingPath") false)
    (else
      (if (`self.IsMoving`)
        (set `self.IsMoving` false)
        (`self.K2_SetActorLocation` (`self.K2_GetActorLocation` (`|GetArrayItem` (`self.TargetList`) (`self.CurrentPoint`))))
        (else
          (set `self.IsMoving` true)))
      (`BlackboardComponent.SetValueAsBool` (`AIBlueprintHelperLibrary.GetBlackboard` null) (`KismetStringLibrary.Conv_StringToName` "IsFollowingPath") (`self.IsMoving`)))))

(event `/Game/Blueprint/BPI_WiredActor.ResetActor`
  (bind _returnvalue (`AIBlueprintHelperLibrary.GetBlackboard` null))
  ;[1 1 1] Reset
  (`self.K2_SetActorTransform` (`self.Transofrm`))
  (set `self.Action_WTB` (`self.Action WTBReset`))
  (set `self.Action_Kill` (`self.Action KillReset`))
  (set `self.PlayerRef` (`self.Player RefReset`))
  (set `self.TargetList` (`self.Target ListReset`))
  (set `self.TargetPointMap` (`self.Target Point MapReset`))
  (set `self.CurrentPoint` (`self.Current PointReset`))
  (set `self.IsMoving` (`self.Is MovingReset`))
  (set `self.EnableMoveAtStart` (`self.Enable Move at StartReset`))
  (`BlackboardComponent.SetValueAsBool` _returnvalue (`KismetStringLibrary.Conv_StringToName` "isTrackingPlayer") false)
  (`BlackboardComponent.SetValueAsBool` _returnvalue (`KismetStringLibrary.Conv_StringToName` "IsFollowingPath") false)
  (`self.Reset`))

(fn `UserConstructionScript`
  (bind _returnvalue (`AddComponent|NODE_AddSplineComponent-3`))
  (`KismetArrayLibrary.Array_AddUnique` (`self.TargetPointMap`) (`self.K2_GetActorLocation`))
  (for _array_element (`self.TargetList`)
    (`/Engine/EditorBlueprintResources/StandardMacros.IsValid` _array_element
      (:`Is Valid`
        (bind _returnvalue_2 (`KismetArrayLibrary.Array_AddUnique` (`self.TargetPointMap`) (`self.K2_GetActorLocation` _array_element)))
        (`TextRenderComponent.K2_SetText` (`/Game/Blueprint/PATHPOINT.TargetIndex` _array_element) (`KismetTextLibrary.Conv_IntToText` _returnvalue_2)))))
  (`SplineComponent.SetSplinePoints` _returnvalue (`self.TargetPointMap`) "World" true))