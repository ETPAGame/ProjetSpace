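; BP_ButtonRed is a one-shot button that triggers the actors wired to it.
; The first Interaction event swaps the button to a green emissive material and sends WiredActionMessage to every WiredItems entry that implements BPI_WiredActor.
; The construction script adds a two-point spline from each valid wired actor to the button's root, tracing the connections.
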(event `/Game/Inputs/BPI_Interact.Interaction`
  (`/Engine/EditorBlueprintResources/StandardMacros.DoOnce` false
    (:`Completed`
      (`PrimitiveComponent.SetMaterial` (`self.Button`) 0 "/Game/DevMapContent/M_TEMP_GreenEmissive.M_TEMP_GreenEmissive")
      (for _array_element (`self.WiredItems`)
        (if (`KismetSystemLibrary.DoesImplementInterface` _array_element "/Game/Inputs/BPI_WiredActor.BPI_WiredActor_C")
          (message `/Game/Inputs/BPI_WiredActor.WiredAction` _array_element))))))

(fn `UserConstructionScript`
  (for _array_element (`self.WiredItems`)
    (`/Engine/EditorBlueprintResources/StandardMacros.IsValid` _array_element
      (:`Is Valid`
        (bind _returnvalue (`AddComponent|NODE_AddSplineComponent-0`))
        (`SplineComponent.SetSplinePoints` _returnvalue (`|MakeArray` (`self.K2_GetActorLocation` _array_element) (`SceneComponent.K2_GetComponentLocation` (`self.DefaultSceneRoot`))) "World" true)))))