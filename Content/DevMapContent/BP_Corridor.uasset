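; Procedural corridor actor that builds a straight hallway along Y with flickering ceiling lights.
; The construction script repeats floor, side and top meshes per Size step, adding fixture meshes and a point light where the Lights entry passes.
; It clears and resizes Lights first, and never stores the created lights there.
; BeginPlay calls Flicker per Lights entry, using one shared timeline to randomise clamped intensity at curve peaks.
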(event `self.ReceiveBeginPlay`
  (for _array_element (`self.Lights`)
    (`self.flicker` _array_element)
    (`KismetSystemLibrary.PrintString` "Hello")))

(event `flicker`
  (params (Target :type "LightComponent Object Reference"))
  (bind _intensity (`LightComponentBase.Intensity` Target))
  (bind (_direction _newtrack_0) (`Timeline|Timeline_0`)
    (:`Update`
      (if (> _newtrack_0 0.9)
        (`LightComponent.SetIntensity` Target (`KismetMathLibrary.FClamp` (`KismetMathLibrary.RandomFloatInRange` (- _intensity 3000.0) (+ 3000.0 _intensity)) 0.0 3000.0))))))

(fn `UserConstructionScript`
  (`KismetArrayLibrary.Array_Clear` (`self.Lights`))
  (`KismetArrayLibrary.Array_Resize` (`self.Lights?`) (`self.Size`))
  (for _index (range (+ (`self.Size`) 1))
    (set `self.Index` _index)
    (`|ExecutionSequence`
      (:`then_0`
        ;[1 1 1] plane
        (`AddComponent|NODE_AddStaticMeshComponent-1` :`RelativeTransform` (`KismetMathLibrary.MakeTransform` (`KismetMathLibrary.MakeVector` 0.0 (+ 0.0 (* (`self.Index`) 100.0))))))
      (:`then_1`
        (`AddComponent|NODE_AddStaticMeshComponent-4` :`RelativeTransform` (`KismetMathLibrary.MakeTransform` (`KismetMathLibrary.MakeVector` -350.0 (+ 0.0 (* (`self.Index`) 100.0)) 350.0) (struct))))
      (:`then_2`
        (`AddComponent|NODE_AddStaticMeshComponent-3` :`RelativeTransform` (`KismetMathLibrary.MakeTransform` (`KismetMathLibrary.MakeVector` 350.0 (+ 0.0 (* (`self.Index`) 100.0)) 350.0) (struct))))
      (:`then_3`
        (`AddComponent|NODE_AddStaticMeshComponent-2` :`RelativeTransform` (`KismetMathLibrary.MakeTransform` (`KismetMathLibrary.MakeVector` 0.0 (+ 0.0 (* (`self.Index`) 100.0)) 700.0) (struct))))
      (:`then_4`
        (if (`|GetArrayItem` (`self.Lights?`) (`self.Index`))
          (`|ExecutionSequence`
            (:`then_0`
              (`AddComponent|NODE_AddStaticMeshComponent-5` :`RelativeTransform` (`KismetMathLibrary.MakeTransform` (`KismetMathLibrary.MakeVector` 0.0 (+ (`KismetMathLibrary.Conv_IntToDouble` (* (`self.Index`) 700)) 90.0) 700.0) (struct :`Roll` 90.0) (0.2 1.0 5.0))))
            (:`then_1`
              (`AddComponent|NODE_AddStaticMeshComponent-6` :`RelativeTransform` (`KismetMathLibrary.MakeTransform` (`KismetMathLibrary.MakeVector` 0.0 (+ (`KismetMathLibrary.Conv_IntToDouble` (* (`self.Index`) 700)) 90.0) 710.0) (struct :`Roll` 90.0) (1.25 1.25 1.25))))
            (:`then_2`
              (`AddComponent|NODE_AddPointLightComponent-2` :`RelativeTransform` (`KismetMathLibrary.MakeTransform` (`KismetMathLibrary.MakeVector` 0.0 (+ (`KismetMathLibrary.Conv_IntToDouble` (* (`self.Index`) 700)) 90.0) 700.0) (struct :`Pitch` -90.0 :`Yaw` 90.0) (10.0 10.0 0.3))))))))))