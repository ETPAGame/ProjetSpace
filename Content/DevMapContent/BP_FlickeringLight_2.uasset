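; A flickering light actor that drives two rect lights, the second at half the intensity of the first.
; A randomized timer loop alternately plays and reverses a timeline, whose updates feed a randomized sine into the intensity.
; Each finished flicker restores the default intensity and schedules the next.
; Switch toggles the lights off, suppressing flicker, or restarts the loop; its delayed demo sequence is never run.
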(event `self.ReceiveBeginPlay`
  ;[1 1 1] DEMO
  (`self.Start Flicker Loop`))

(event `Switch`
  ;[1 1 1] Switch Mode
  (`/Engine/EditorBlueprintResources/StandardMacros.FlipFlop`
    (:`A`
      (set `self.ForceStop?` true)
      (`self.Set All Intensity` 0.0))
    (:`B`
      (set `self.ForceStop?` false)
      (`self.Start Flicker Loop`))))

(event `Flicker`
  ;[1 1 1] Flicker
  (if (not (`self.ForceStop?`))
    (`/Engine/EditorBlueprintResources/StandardMacros.FlipFlop`
      (:`A`
        (bind (_direction _newtrack_0) (`Timeline|Flick` :!label _label)
          (:`Update`
            (if (not (`self.ForceStop?`))
              (`self.Set All Intensity` (* (`KismetMathLibrary.MapRangeClamped` (`KismetMathLibrary.Sin` (* (`KismetMathLibrary.RandomFloatInRange` 0.5 3.0) _newtrack_0)) -1.0 1.0 2000.0 5000.0) (`KismetMathLibrary.RandomFloatInRange` 0.0 1.0)))))
          (:`Finished`
            (`self.Set All Intensity` (`self.Default Intensity`))
            (`KismetSystemLibrary.K2_SetTimerDelegate` (delegate `Flicker`) (`KismetMathLibrary.RandomFloatInRange` 1.0 5.0) :!label _label_2))))
      (:`B`
        (goto _label :!via `Reverse`)))))

(event `Start Flicker Loop`
  ;[1 1 1] Flicker
  (goto _label_2))

(fn `Set All Intensity`
  (params (Intensity :type "Float (double-precision)"))
  (`LightComponent.SetIntensity` (`self.RectLight`) Intensity)
  (`LightComponent.SetIntensity` (`self.RectLight1`) (/ Intensity 2.0)))

(fn `UserConstructionScript`
  (`self.Set All Intensity` (`self.Default Intensity`)))