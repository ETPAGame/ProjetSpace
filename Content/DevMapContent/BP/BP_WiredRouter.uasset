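; Wired router actor that relays an action request to one of the actors linked in its WiredActors array.
; SendRequest takes an index and calls WiredActionMessage on that entry, without a validity check.
; The construction script adds a world-space spline from each valid linked actor's location to the router's Billboard, tracing the wiring.
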(event `Send Request`
  (params (To :type Integer))
  (message `/Game/Inputs/BPI_WiredActor.WiredAction` (`|GetArrayItem` (`self.WiredActors`) To)))

(fn `UserConstructionScript`
  (for _array_element (`self.WiredActors`)
    (`/Engine/EditorBlueprintResources/StandardMacros.IsValid` _array_element
      (:`Is Valid`
        (bind _returnvalue (`AddComponent|NODE_AddSplineComponent-0`))
        (`SplineComponent.SetSplinePoints` _returnvalue (`|MakeArray` (`self.K2_GetActorLocation` _array_element) (`SceneComponent.K2_GetComponentLocation` (`self.Billboard`))) "World" true)))))