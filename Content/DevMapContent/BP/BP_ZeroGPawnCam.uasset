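; Zero-gravity first-person pawn that drifts, grabs surfaces on contact and launches along the camera's forward vector.
; Mouse look flips roll, yaw and pitch input near the vertical poles to allow looking through full loops.
; Capsule hits on the grab channel stop movement, face the surface and clamp yaw; left-click zooms FOV, launching on release.
; It also sphere-traces for BPI_Interact targets and can replace itself with a spawned BP_FirstPersonCharacter.
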(event `EnhancedInput|/Game/Inputs/IA_Interaction`
  (params (ActionValue :type Boolean) (ElapsedSeconds :type "Float (double-precision)") (TriggeredSeconds :type "Float (double-precision)") (InputAction :type "InputAction Object Reference" :default "/Game/Inputs/IA_Interaction.IA_Interaction"))
  (bind _camera (`self.Camera`))
  (bind _returnvalue (`SceneComponent.K2_GetComponentLocation` _camera))
  ;[1 1 1] Interaction Input
  (:`Triggered`
    (`/Engine/EditorBlueprintResources/StandardMacros.DoOnce` false :!label _label
      (:`Completed`
        (bind _outhits (`KismetSystemLibrary.SphereTraceMulti` :`Start` _returnvalue :`End` (+ _returnvalue (* (`SceneComponent.GetForwardVector` _camera) 300.0)) :`Radius` 20.0 :`TraceChannel` "TraceTypeQuery3" :`DrawDebugType` "ForDuration"))
        (for _array_element _outhits
          (if (`KismetSystemLibrary.DoesImplementInterface` (`.HitActor` (`GameplayStatics.BreakHitResult` _array_element)) "/Game/Inputs/BPI_Interact.BPI_Interact_C")
            (message `/Game/Inputs/BPI_Interact.Interaction` (`.HitActor` (`GameplayStatics.BreakHitResult` _array_element)))
            (break))))))
  (:`Completed`
    (goto _label :!via `Reset`)))

(event `InputAxis|LookUp`
  (params (AxisValue :type "Float (single-precision)"))
  ;[1 1 1] ZeroG Free view
  (`self.InputPitch` AxisValue))

(event `InputAxis|Turn`
  (params (AxisValue :type "Float (single-precision)"))
  ;[1 1 1] ZeroG Free view
  (`self.InputYaw` AxisValue))

(event `InputPitch`
  (params (Value :type "Float (double-precision)"))
  (bind (_returnvalue_roll _returnvalue_pitch _returnvalue_yaw) (`KismetMathLibrary.BreakRotator` (`SceneComponent.K2_GetComponentRotation` (`self.Camera`))))
  ;[1 1 1] ZeroG Free view
  (`self.PitchManager` _returnvalue_pitch Value)
  (`self.K2_SetActorRotation` (`KismetMathLibrary.MakeRotator` (`self.RollValue`) (+ (* Value (`self.Invert Axis`)) _returnvalue_pitch) _returnvalue_yaw)))

(event `self.ReceiveTick`
  (params (DeltaSeconds :type "Float (single-precision)"))
  (bind (_returnvalue_roll _returnvalue_pitch _returnvalue_yaw) (`KismetMathLibrary.BreakRotator` (`SceneComponent.K2_GetComponentRotation` (`self.Camera`))))
  (`KismetSystemLibrary.PrintString` (`KismetStringLibrary.Concat_StrStr` "0Grab? : " (`KismetStringLibrary.Conv_BoolToString` (`self.ZeroG_IsGrab?`))) true true (struct :`R` 1.0 :`G` 0.070155 :`B` 0.030354 :`A` 1.0) 0.0)
  (`KismetSystemLibrary.PrintString` (`KismetStringLibrary.Concat_StrStr` "Roll : " (`KismetStringLibrary.Conv_DoubleToString` _returnvalue_roll)) true true (struct :`R` 1.0 :`B` 0.013355 :`A` 1.0) 0.0)
  (`KismetSystemLibrary.PrintString` (`KismetStringLibrary.Concat_StrStr` "Pitch : " (`KismetStringLibrary.Conv_DoubleToString` _returnvalue_pitch)) true true (struct :`G` 1.0 :`B` 0.012901 :`A` 1.0) 0.0)
  (`KismetSystemLibrary.PrintString` (`KismetStringLibrary.Concat_StrStr` "Yaw :" (`KismetStringLibrary.Conv_DoubleToString` _returnvalue_yaw)) true true (struct :`G` 0.66 :`B` 1.0 :`A` 1.0) 0.0))

(event `self.ReceiveBeginPlay`
  (bind _returnvalue (`GameplayStatics.GetPlayerCameraManager` 0))
  (set `self.DefaultTransformMesh` (`SceneComponent.GetRelativeTransform` (`self.SkeletalMesh`)))
  (set `self.DefaultYawMin` (`PlayerCameraManager.ViewYawMin` _returnvalue))
  (set `self.DefaultYawMax` (`PlayerCameraManager.ViewYawMax` _returnvalue)))

(event `InputYaw`
  (params (Value :type "Float (double-precision)"))
  (bind (_returnvalue_roll _returnvalue_pitch _returnvalue_yaw) (`KismetMathLibrary.BreakRotator` (`SceneComponent.K2_GetComponentRotation` (`self.Camera`))))
  ;[1 1 1] ZeroG Free view
  (`self.K2_SetActorRotation` (`KismetMathLibrary.MakeRotator` (`self.RollValue`) _returnvalue_pitch (+ _returnvalue_yaw (* Value (* (`self.Invert Axis`) -1.0))))))

(event `Key|LeftMouseButton`
  (params (Key :type "Key Structure"))
  (bind _zerog_isgrab_ (`self.ZeroG_IsGrab?`))
  ;[1 1 1] ZeroG Actions
  (:`Pressed`
    (if _zerog_isgrab_
      (bind (_direction _newtrack_0) (`Timeline|Timeline_0` :!label _label_2)
        (:`Update`
          (`CameraComponent.SetFieldOfView` (`self.Camera`) (`KismetMathLibrary.Lerp` 100.0 75.0 _newtrack_0))))))
  (:`Released`
    (if _zerog_isgrab_
      (`self.ZeroG_Launch`)
      (goto _label_2 :!via `Reverse`))))

(event `InputRoll`
  (params (Value :type "Float (double-precision)"))
  (bind (_returnvalue_roll _returnvalue_pitch _returnvalue_yaw) (`KismetMathLibrary.BreakRotator` (`self.K2_GetActorRotation`)))
  ;[1 1 1] ZeroG Free view
  (`self.K2_SetActorRotation` (`KismetMathLibrary.MakeRotator` (+ Value _returnvalue_roll) _returnvalue_pitch _returnvalue_yaw)))

(event `self.Capsule.OnComponentHit`
  (params (HitComponent :type "PrimitiveComponent Object Reference") (OtherActor :type "Actor Object Reference") (OtherComp :type "PrimitiveComponent Object Reference") (NormalImpulse :type "Vector Structure") (Hit :type "HitResult Structure (by ref)"))
  ;[1 1 1] ZeroG Grab/Launch
  (if (== (`|GetEnumeratorName` (`self.ZeroG_GrabChannel`)) (`|GetEnumeratorName` (`PrimitiveComponent.GetCollisionObjectType` OtherComp)))
    (`/Engine/EditorBlueprintResources/StandardMacros.DoOnce` false :!label _label_3
      (:`Completed`
        (`self.ZeroG_LockOnWall` (`.ImpactPoint` (`GameplayStatics.BreakHitResult` Hit)))))))

(event `ZeroG_Launch`
  (bind _skeletalmesh (`self.SkeletalMesh`))
  ;[1 1 1] ZeroG Grab/Launch
  (set `MovementComponent.Velocity` (* (`SceneComponent.GetForwardVector` (`self.Camera`)) 500.0) (`self.FloatingPawnMovement`))
  (set `self.ZeroG_IsGrab?` false)
  (`SceneComponent.K2_AttachToComponent` _skeletalmesh (`self.Camera`) "None" "SnapToTarget" "SnapToTarget" "SnapToTarget" true)
  (`SceneComponent.K2_SetRelativeTransform` _skeletalmesh (`self.DefaultTransformMesh`) false false)
  (`self.ClampYawAxis` 0.0 0.0 true)
  (goto _label_3 :!via `Reset`))

(event `ZeroG_LockOnWall`
  (params (HitPoint :type "Vector Structure"))
  (bind _returnvalue_roll (`KismetMathLibrary.BreakRotator` (`self.K2_GetActorRotation`)))
  (bind _camera (`self.Camera`))
  (bind _floatingpawnmovement (`self.FloatingPawnMovement`))
  (bind (_returnvalue_roll_2 _returnvalue_pitch _returnvalue_yaw) (`KismetMathLibrary.BreakRotator` (`KismetMathLibrary.FindLookAtRotation` (`SceneComponent.K2_GetComponentLocation` _camera) HitPoint)))
  ;[1 1 1] ZeroG Grab/Launch
  (set `MovementComponent.Velocity` (0.0 0.0 0.0) _floatingpawnmovement)
  (`MovementComponent.StopMovementImmediately` _floatingpawnmovement)
  (set `self.ZeroG_IsGrab?` true)
  (bind (_direction _newtrack_0) (`Timeline|Timeline_1` :!via `PlayFromStart`)
    (:`Update`
      (bind _returnvalue (`KismetMathLibrary.RLerp` (`SceneComponent.K2_GetComponentRotation` _camera) (`KismetMathLibrary.MakeRotator` _returnvalue_roll _returnvalue_pitch _returnvalue_yaw) _newtrack_0 true))
      (`self.K2_SetActorRotation` _returnvalue))
    (:`Finished`
      (`SceneComponent.K2_DetachFromComponent` (`self.SkeletalMesh`) "KeepWorld" "KeepWorld" "KeepWorld" true)
      (`self.ClampYawAxis` (.yaw _returnvalue) 135.0)
      (set `MovementComponent.Velocity` (0.0 0.0 0.0) (`self.FloatingPawnMovement`)))))

(event `RePossessPlayer`
  (bind (_returnvalue_roll _returnvalue_pitch _returnvalue_yaw) (`KismetMathLibrary.BreakRotator` (`self.K2_GetActorRotation`)))
  (bind _returnvalue (`GameplayStatics.GetPlayerController` 0))
  (bind _skeletalmesh (`self.SkeletalMesh`))
  ;[1 1 1] Detach if Grab
  (if (`self.ZeroG_IsGrab?`)
    (set `self.ZeroG_IsGrab?` false)
    (`SceneComponent.K2_AttachToComponent` _skeletalmesh (`self.Camera`) "None" "SnapToTarget" "SnapToTarget" "SnapToTarget" true)
    (`SceneComponent.K2_SetRelativeTransform` _skeletalmesh (`self.DefaultTransformMesh`) false false))
  ;[1 1 1] BP FP Chara Repossess
  (`KismetSystemLibrary.PrintString` "Repo")
  (`SceneComponent.SetVisibility` (`self.SkeletalMesh`) false false)
  (bind _returnvalue_2 (`|SpawnActorFromClass` "/Game/FirstPerson/Blueprints/BP_FirstPersonCharacter.BP_FirstPersonCharacter_C" (`KismetMathLibrary.MakeTransform` (`self.K2_GetActorLocation`) (`KismetMathLibrary.MakeRotator` 0.0 _returnvalue_pitch _returnvalue_yaw)) "AdjustIfPossibleButAlwaysSpawn" "OverrideRootScale" null null))
  (`PlayerController.SetViewTargetWithBlend` _returnvalue _returnvalue_2 0.1 "VTBlend_Linear" 0.0 false)
  (`KismetSystemLibrary.Delay` 0.1)
  (`Controller.Possess` _returnvalue _returnvalue_2)
  (`self.ClampYawAxis` 0.0 0.0 true)
  (`self.K2_DestroyActor`))

(fn `ClampYawAxis`
  (params (`Yaw Value` :type "Float (double-precision)") (Offset :type "Float (double-precision)") (Reset :type Boolean))
  (bind _returnvalue (`GameplayStatics.GetPlayerCameraManager` 0))
  (if (not Reset)
    (set `PlayerCameraManager.ViewYawMin` (- `Yaw Value` Offset) _returnvalue)
    (set `PlayerCameraManager.ViewYawMax` (+ `Yaw Value` Offset) _returnvalue)
    (else
      (set `PlayerCameraManager.ViewYawMin` (`self.DefaultYawMin`) _returnvalue)
      (set `PlayerCameraManager.ViewYawMax` (`self.DefaultYawMax`) _returnvalue))))

(fn `PitchManager`
  (params (`Current Pitch Value` :type "Float (double-precision)") (`Axis Input` :type "Float (double-precision)"))
  (bind _output (`self.Set to Positive` `Axis Input`))
  (if (not (`self.IsRolling`))
    (bind _returnvalue (+ _output 1.0))
    (if (`KismetMathLibrary.NearlyEqual_FloatFloat` `Current Pitch Value` 90.0 _returnvalue)
      (if (< `Axis Input` -0.1)
        (`/Engine/EditorBlueprintResources/StandardMacros.DoOnce` false :!label _label
          (:`Completed`
            (set `self.RollValue` -180.0)
            (set `self.IsRolling` true)
            (set `self.Invert Axis` 1.0)
            (`self.K2_AddActorWorldRotation` (`KismetMathLibrary.MakeRotator` 0.0 0.0 180.0))
            (goto _label_2 :!via `Reset`))))
      (elif (`KismetMathLibrary.NearlyEqual_FloatFloat` `Current Pitch Value` -90.0 _returnvalue)
        (if (> `Axis Input` 0.1)
          (goto _label))))
    (elif (`KismetMathLibrary.NearlyEqual_FloatFloat` `Current Pitch Value` 90.0 _returnvalue)
      (if (> `Axis Input` 0.1)
        (`/Engine/EditorBlueprintResources/StandardMacros.DoOnce` false :!label _label_2
          (:`Completed`
            (set `self.RollValue` 0.0)
            (set `self.IsRolling` false)
            (set `self.Invert Axis` -1.0)
            (`self.K2_AddActorWorldRotation` (`KismetMathLibrary.MakeRotator` 0.0 0.0 180.0))
            (goto _label :!via `Reset`))))
      (elif (`KismetMathLibrary.NearlyEqual_FloatFloat` `Current Pitch Value` -90.0 _output)
        (if (< `Axis Input` -0.1)
          (goto _label_2))))))

(fn `Set to Positive`
  (params (Input :type "Float (double-precision)"))
  (returns (Output :type "Float (double-precision)"))
  (set `self.SetPositiveValue` Input)
  (if (< (`self.SetPositiveValue`) 0.0)
    (set `self.SetPositiveValue` (* (`self.SetPositiveValue`) -1.0)))
  (return (`self.SetPositiveValue`)))

(fn `UserConstructionScript`)