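; BP_DoubleDoors is a sliding double door that opens when the first-person character or zero-G camera pawn enters its trigger box and closes when it leaves.
; A timeline lerps the right leaf along Y to a configurable OpenDestination, mirrors the left by negation, and reverses to close.
; A Locked flag blocks both actions until WiredAction clears it.
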(event `/Game/Inputs/BPI_WiredActor.WiredAction`
  (set `self.Locked?` false))

(event `self.Box.OnComponentBeginOverlap`
  (params (OverlappedComponent :type "PrimitiveComponent Object Reference") (OtherActor :type "Actor Object Reference") (OtherComp :type "PrimitiveComponent Object Reference") (OtherBodyIndex :type Integer) (bFromSweep :type Boolean) (SweepResult :type "HitResult Structure (by ref)"))
  (cast `/Game/FirstPerson/Blueprints/BP_FirstPersonCharacter` OtherActor
    (:`then`
      _)
    (:`CastFailed`
      (cast `/Game/DevMapContent/BP/BP_ZeroGPawnCam` OtherActor)))
  (if (not (`self.Locked?`))
    (`self.Open`)))

(event `self.Box.OnComponentEndOverlap`
  (params (OverlappedComponent :type "PrimitiveComponent Object Reference") (OtherActor :type "Actor Object Reference") (OtherComp :type "PrimitiveComponent Object Reference") (OtherBodyIndex :type Integer))
  (cast `/Game/FirstPerson/Blueprints/BP_FirstPersonCharacter` OtherActor
    (:`then`
      _)
    (:`CastFailed`
      (cast `/Game/DevMapContent/BP/BP_ZeroGPawnCam` OtherActor)))
  (if (not (`self.Locked?`))
    (`self.Close`)))

(event `Open`
  (bind (_direction _alpha) (`Timeline|DoorsTimeline` :!label _label)
    (:`Update`
      (bind _returnvalue (`KismetMathLibrary.VLerp` (0.0 80.0 0.0) (`KismetMathLibrary.MakeVector` 0.0 (`self.OpenDestination`)) _alpha))
      (`SceneComponent.K2_SetRelativeLocation` (`self.DoorR`) _returnvalue false false)
      (`SceneComponent.K2_SetRelativeLocation` (`self.DoorL`) (`KismetMathLibrary.NegateVector` _returnvalue) false false))))

(event `Close`
  (goto _label :!via `Reverse`))

(fn `UserConstructionScript`)