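; BP_PorteSAS is a door that slides vertically when the first-person character enters or leaves its Box trigger.
; Both overlap events call the same OpenDoor event, which eases the Cube to a new relative height over half a second.
; The target is computed as the clamped absolute difference between current Z and the travel height, acting as a stateless toggle that assumes the door is at an end position.
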(event `self.Box.OnComponentBeginOverlap`
  (params (OverlappedComponent :type "PrimitiveComponent Object Reference") (OtherActor :type "Actor Object Reference") (OtherComp :type "PrimitiveComponent Object Reference") (OtherBodyIndex :type Integer) (bFromSweep :type Boolean) (SweepResult :type "HitResult Structure (by ref)"))
  (cast `/Game/FirstPerson/Blueprints/BP_FirstPersonCharacter` OtherActor)
  (`self.OpenDoor`))

(event `self.Box.OnComponentEndOverlap`
  (params (OverlappedComponent :type "PrimitiveComponent Object Reference") (OtherActor :type "Actor Object Reference") (OtherComp :type "PrimitiveComponent Object Reference") (OtherBodyIndex :type Integer))
  (cast `/Game/FirstPerson/Blueprints/BP_FirstPersonCharacter` OtherActor)
  (`self.OpenDoor`))

(event `OpenDoor`
  (bind _cube (`self.Cube`))
  (bind (_relativelocation_x _relativelocation_y _relativelocation_z) (`KismetMathLibrary.BreakVector` (`SceneComponent.RelativeLocation` _cube)))
  (`KismetSystemLibrary.MoveComponentTo` _cube (`KismetMathLibrary.MakeVector` _relativelocation_x _relativelocation_y (`KismetMathLibrary.FClamp` (`KismetMathLibrary.Abs` (- _relativelocation_z 200.0)) 0.0 200.0)) (struct) true true 0.5))

(fn `UserConstructionScript`)