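; Manager that toggles the player between the first-person character and the zero-gravity camera pawn through a single WiredAction event.
; When controlling BP_FirstPersonCharacter off its zero-G cooldown, the event calls Pawner on it.
; When controlling BP_ZeroGPawnCam, it calls RePossessPlayer to return control.
; Two DoOnce gates reset each other, so each switch fires only once until the opposite one runs.
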(event `/Game/Inputs/BPI_WiredActor.WiredAction`
  (bind _returnvalue (`Controller.K2_GetPawn` (`GameplayStatics.GetPlayerController` 0)))
  (bind _asbp_first_person_character (cast `/Game/FirstPerson/Blueprints/BP_FirstPersonCharacter` _returnvalue)
    (:`then`
      (if (not (`/Game/FirstPerson/Blueprints/BP_FirstPersonCharacter.ZeroG_Cooldown` _asbp_first_person_character))
        (`/Engine/EditorBlueprintResources/StandardMacros.DoOnce` false :!label _label
          (:`Completed`
            (`/Game/FirstPerson/Blueprints/BP_FirstPersonCharacter.Pawner` _asbp_first_person_character)
            (goto _label_2 :!via `Reset`)))))
    (:`CastFailed`
      (bind _asbp_zero_gpawn_cam (cast `/Game/DevMapContent/BP_ZeroGPawnCam` _returnvalue))
      (`/Engine/EditorBlueprintResources/StandardMacros.DoOnce` true :!label _label_2
        (:`Completed`
          (`/Game/DevMapContent/BP_ZeroGPawnCam.RePossessPlayer` _asbp_zero_gpawn_cam)
          (goto _label :!via `Reset`))))))

(fn `UserConstructionScript`)