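; Zero-G camera pawn in dev map content that gives pitch, yaw and roll control, with no movement logic.
; LookUp (inverted) and Turn axes add to the camera's world pitch and yaw, while held A/E keys roll the actor every tick.
; Each input rebuilds the actor rotation from Euler components rather than applying local rotations, and roll speed is frame-rate dependent.
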(event `self.ReceiveTick`
  (params (DeltaSeconds :type "Float (single-precision)"))
  (if (`self.IsRolling`)
    (`self.InputRoll` (`self.RollValue`))))

(event `Key|A`
  (params (Key :type "Key Structure"))
  (:`Pressed`
    (set `self.RollValue` -1.0)
    (set `self.IsRolling` true :!label _label))
  (:`Released`
    (set `self.IsRolling` false :!label _label_2)))

(event `Key|E`
  (params (Key :type "Key Structure"))
  (:`Pressed`
    (set `self.RollValue` 1.0)
    (goto _label))
  (:`Released`
    (goto _label_2)))

(event `InputAxis|LookUp`
  (params (AxisValue :type "Float (single-precision)"))
  (`self.InputPitch` AxisValue))

(event `InputAxis|Turn`
  (params (AxisValue :type "Float (single-precision)"))
  (`self.InputYaw` AxisValue))

(event `InputPitch`
  (params (Value :type "Float (double-precision)"))
  (bind (_returnvalue_roll _returnvalue_pitch _returnvalue_yaw) (`KismetMathLibrary.BreakRotator` (`SceneComponent.K2_GetComponentRotation` (`self.Camera`))))
  (`self.K2_SetActorRotation` (`KismetMathLibrary.MakeRotator` _returnvalue_roll (+ (* Value -1.0) _returnvalue_pitch) _returnvalue_yaw)))

(event `InputYaw`
  (params (Value :type "Float (double-precision)"))
  (bind (_returnvalue_roll _returnvalue_pitch _returnvalue_yaw) (`KismetMathLibrary.BreakRotator` (`SceneComponent.K2_GetComponentRotation` (`self.Camera`))))
  (`self.K2_SetActorRotation` (`KismetMathLibrary.MakeRotator` _returnvalue_roll _returnvalue_pitch (+ _returnvalue_yaw Value))))

(event `InputRoll`
  (params (Value :type "Float (double-precision)"))
  (bind (_returnvalue_roll _returnvalue_pitch _returnvalue_yaw) (`KismetMathLibrary.BreakRotator` (`self.K2_GetActorRotation`)))
  (`self.K2_SetActorRotation` (`KismetMathLibrary.MakeRotator` (+ Value _returnvalue_roll) _returnvalue_pitch _returnvalue_yaw)))

(fn `UserConstructionScript`)