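; Trigger volume that plays a one-shot cinematic when the zero-G pawn or first-person character enters, once armed by WiredAction.
; It disables input, blends to the cinematic camera, plays the level sequence and waits out its duration.
; It then teleports the player, restores camera and input, and can switch gravity mode and HUD through BP_ZeroGravityManager.
; An optional hallucination post-process brackets the sequence on the first-person character.
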(event `PlayCine`
  (bind _returnvalue (`GameplayStatics.GetPlayerController` 0))
  (bind _returnvalue_2 (`GameplayStatics.GetPlayerController` 0))
  (bind (_transformendcinematique_loctp _transformendcinematique_rottp) (break `/Game/Teleport_Struct` (`self.TransformEndCinematique`)))
  (bind _sequenceplayer (`LevelSequenceActor.SequencePlayer` (`self.LevelSequenceRef`)))
  (bind _returnvalue_3 (`TimeManagementBlueprintLibrary.Conv_QualifiedFrameTimeToSeconds` (`MovieSceneSequencePlayer.GetDuration` _sequenceplayer)))
  (`self.DisableInput` (`self.PlayerRef`) _returnvalue_2)
  (set `self.CamRefReturn` (`Controller.GetViewTarget` _returnvalue_2))
  (`PlayerController.SetViewTargetWithBlend` (`GameplayStatics.GetPlayerController` 0) (`self.CineCamRef`) (`self.Blend Time`) "VTBlend_Linear" 0.0 false)
  (`MovieSceneSequencePlayer.Play` _sequenceplayer)
  (set `self.HalluLenght` _returnvalue_3)
  (`KismetSystemLibrary.Delay` _returnvalue_3)
  (`self.K2_TeleportTo` (`self.PlayerRef`) _transformendcinematique_loctp _transformendcinematique_rottp)
  (if (`self.hallu?`)
    (`/Game/Blueprint/BP_FirstPersonCharacter.hallu1PPEnter` (`self.FirstPerson Ref`) (`self.HalluLenght`) true))
  (`PlayerController.SetViewTargetWithBlend` (`GameplayStatics.GetPlayerController` 0) (`self.CamRefReturn`) (`self.Blend Time`) "VTBlend_Linear" 0.0 false)
  (`self.EnableInput` (`self.PlayerRef`) (`GameplayStatics.GetPlayerController` 0))
  (if (`self.ToPawn?`)
    (bind _asbp_player_controller (cast `/Game/Blueprint/BP_PlayerController` _returnvalue))
    (bind _returnvalue_4 (`GameplayStatics.GetActorOfClass` "/Game/Blueprint/BP_ZeroGravityManager.BP_ZeroGravityManager_C" :!label _label))
    (`/Game/Blueprint/BP_ZeroGravityManager.Switch` _returnvalue_4)
    (bind _hudref (`/Game/Blueprint/BP_PlayerController.HUDRef` _asbp_player_controller))
    (`/Game/WPB_HUDInGame.SwitchBetweenGlypheAndNoGlyphe` _hudref true)
    (`/Game/WPB_HUDInGame.Set0GravityPorteOut` _hudref true)
    (elif (`self.toFirstPerson`)
      (cast `/Game/Blueprint/BP_PlayerController` _returnvalue
        (:`then`
          (goto _label))
        (:`CastFailed`
          (bind _returnvalue_5 (`GameplayStatics.GetActorOfClass` "/Game/Blueprint/BP_ZeroGravityManager.BP_ZeroGravityManager_C"))
          (`/Game/Blueprint/BP_ZeroGravityManager.SwitchtoFirstPerson` _returnvalue_5)
          (bind _returnvalue_6 (`GameplayStatics.GetActorOfClass` "/Game/Blueprint/BP_FirstPersonCharacter.BP_FirstPersonCharacter_C"))
          (`/Game/Blueprint/BP_FirstPersonCharacter.GravitySwitch` _returnvalue_6)
          (`/Game/WPB_HUDInGame.SwitchBetweenGlypheAndNoGlyphe` _hudref false))))))

(event `self.Box.OnComponentBeginOverlap`
  (params (OverlappedComponent :type "PrimitiveComponent Object Reference") (OtherActor :type "Actor Object Reference") (OtherComp :type "PrimitiveComponent Object Reference") (OtherBodyIndex :type Integer) (bFromSweep :type Boolean) (SweepResult :type "HitResult Structure (by ref)"))
  (if (`self.isActive?`)
    (bind _asbp_zero_gpawn_cam (cast `/Game/Blueprint/BP_ZeroGPawnCam` OtherActor)
      (:`then`
        (set `self.PlayerRef` _asbp_zero_gpawn_cam))
      (:`CastFailed`
        (bind _asbp_first_person_character (cast `/Game/Blueprint/BP_FirstPersonCharacter` OtherActor))
        (set `self.PlayerRef` _asbp_first_person_character)
        (set `self.FirstPerson Ref` _asbp_first_person_character)))
    (if (not (`self.HasPlay?`))
      (`self.PlayCine`)
      (set `self.HasPlay?` true)
      (if (`self.hallu?`)
        (`/Game/Blueprint/BP_FirstPersonCharacter.hallu1PPEnter` _asbp_first_person_character (`self.HalluLenght`) false)))))

(event `/Game/Blueprint/BPI_WiredActor.WiredAction`
  (set `self.isActive?` true))

(fn `UserConstructionScript`)