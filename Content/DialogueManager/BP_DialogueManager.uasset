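; Dialogue manager that plays voice lines by ID from a dialogue table, with optional subtitles on the first-person character's HUD.
; PlayAudio plays one line at a time, queuing unique IDs requested while busy.
; After each line's delay it follows the line's Next link, otherwise pulls from the queue.
; VoiceLoc plays Player and IA voices in 2D and attaches Enemy voices to the enemy found by GetRef.
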(event `GetRef`
  ;[1 0 0.6776] GetRefs
  (bind _asbp_first_person_character (cast `/Game/Blueprint/BP_FirstPersonCharacter` (`GameplayStatics.GetPlayerCharacter` 0)))
  (set `self.As BP First Person Character` _asbp_first_person_character)
  (set `self.HUDRef` (`/Game/Blueprint/BP_FirstPersonCharacter.HUDRef` _asbp_first_person_character))
  (bind _returnvalue (`GameplayStatics.GetActorOfClass` "/Game/Blueprint/BP_Enemy.BP_Enemy_C"))
  (set `self.EnemyRef` _returnvalue))

(event `PlayAudio`
  (params (IdSound :type Integer))
  (bind _id_sound (`self.Id Sound`))
  (bind _cue (`self.Cue`))
  (bind (_output_text _output_audio _output_delay _output_next _output_voiceloc) (break `/Game/DialogueManager/Struct_Dialogue` (`|GetArrayItem` (`self.DialogueTab`) _id_sound)))
  ;[1 0.053 0] PlaySound
  (if (`self.IsAvailable`)
    (set `self.Id Sound` IdSound)
    (set `self.IsAvailable` false)
    (`|ExecutionSequence`
      (:`then_0`
        ;;[1 1 1] Trigger Subtitle
        (if (`self.Subtitle?`)
          (`self.ShowSubtitle` _id_sound)))
      (:`then_1`
        (`self.VoiceLoc` _output_audio _output_voiceloc))
      (:`then_2`
        ;;[1 1 1] Cue Manager
        (`KismetSystemLibrary.Delay` _output_delay)
        (set `self.IsAvailable` true)
        (if (!= _output_next 0)
          (`self.PlayAudio` _output_next)
          (elif (!= (`KismetArrayLibrary.Array_Length` (`self.Cue`)) 0)
            (bind _output_get (set `self.Temp` (`|GetArrayItem` _cue)))
            (`KismetArrayLibrary.Array_Remove` _cue)
            (`self.PlayAudio` _output_get)))))
    (else
      ;;[1 1 1] AddToCue
      (`KismetArrayLibrary.Array_AddUnique` (`self.Cue`) IdSound))))

(event `ShowSubtitle`
  (params (IdSub :type Integer))
  (bind (_output_text _output_audio _output_delay) (break `/Game/DialogueManager/Struct_Dialogue` (`|GetArrayItem` (`self.DialogueTab`) IdSub)))
  ;[1 0.053 0] PlaySound
  ;;[1 1 1] Sub
  (`/Game/WPB_HUDInGame.ShowSubtitle` (`self.HUDRef`) _output_delay _output_text))

(fn `UserConstructionScript`)

(fn `VoiceLoc`
  (params (VoiceToPlay :type "SoundCue Object Reference") (FromWhere :type "/Game/DialogueManager/Enum_VoiceLocation Enum" :default "Enum_VoiceLocation_MAX"))
  (switch `/Game/DialogueManager/Enum_VoiceLocation` FromWhere
    (:`NewEnumerator0`
      (`GameplayStatics.PlaySound2D` VoiceToPlay 1.0 1.0 0.0 null null :!label _label))
    (:`NewEnumerator1`
      (goto _label))
    (:`NewEnumerator2`
      (bind _returnvalue (`GameplayStatics.SpawnSoundAttached` VoiceToPlay (`Actor.RootComponent` (`self.EnemyRef`)) "None" (0.0 0.0 0.0) (struct) "KeepRelativeOffset" false 1.0 1.0 0.0 null null))
      (`AudioComponent.Play` _returnvalue 0.0))))