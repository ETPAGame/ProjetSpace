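; BP_Salle_Normal is a room with six configurable lab doors that updates the zero-G player's exit objective on entry.
; The construction script uses per-door states to remove doors or set them openable or locked, and records the chosen exit door's world location.
; When the player pawn overlaps the box, that location becomes the pawn's Out target and BP_GPS is activated with a new objective.
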(event `SetOut`
  (bind _asbp_zero_gpawn_cam (cast `/Game/Blueprint/BP_ZeroGPawnCam` (`GameplayStatics.GetPlayerPawn` 0)))
  (set `/Game/Blueprint/BP_ZeroGPawnCam.Out` (`self.LocationOut`) _asbp_zero_gpawn_cam)
  (bind _returnvalue (`GameplayStatics.GetActorOfClass` "/Game/Blueprint/BP_GPS.BP_GPS_C"))
  (`/Game/Blueprint/BP_GPS.Activ` _returnvalue)
  (`/Game/Blueprint/BP_GPS.NewObj` _returnvalue))

(event `self.Box.OnComponentBeginOverlap`
  (params (OverlappedComponent :type "PrimitiveComponent Object Reference") (OtherActor :type "Actor Object Reference") (OtherComp :type "PrimitiveComponent Object Reference") (OtherBodyIndex :type Integer) (bFromSweep :type Boolean) (SweepResult :type "HitResult Structure (by ref)"))
  (cast `/Game/Blueprint/BP_ZeroGPawnCam` OtherActor)
  (`self.SetOut`))

(fn `UserConstructionScript`
  (set `self.PorteChild` (`|MakeArray` (`self.Porte_Labs`) (`self.Porte_Labs3`) (`self.Porte_Labs1`) (`self.Porte_Labs2`) (`self.Porte_Labs4`) (`self.Porte_Labs5`)))
  (bind _output_get (set `self.OutRef` (`|GetArrayItem` (`self.PorteChild`) (`self.PorteOut`))))
  (set `self.LocationOut` (`SceneComponent.K2_GetComponentLocation` _output_get))
  (for (_array_element _array_index) (`self.PorteState`)
    (if (`|EnumEquality` _array_element "NewEnumerator1")
      (bind _output (`|GetArrayItem` (`self.PorteChild`) _array_index))
      (`ActorComponent.K2_DestroyComponent` _output)
      (elif (`|EnumEquality` _array_element "NewEnumerator2")
        (bind _childactor (`ChildActorComponent.ChildActor` _output))
        (bind _asporte_labs (cast `/Game/Test/Porte_Labs` _childactor))
        (set `/Game/Test/Porte_Labs.Openable?` false _asporte_labs)
        (else
          (bind _asporte_labs_2 (cast `/Game/Test/Porte_Labs` _childactor))
          (set `/Game/Test/Porte_Labs.Openable?` true _asporte_labs_2))))))